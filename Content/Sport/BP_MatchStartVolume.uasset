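; BP_MatchStartVolume is a trigger actor that starts a sport match when any actor overlaps it.
; Shortly after BeginPlay it finds the level's sport manager, or logs a warning and spawns a BP_SportManager if none exists.
; On overlap, if its SportData is valid, it logs the sport type and passes the data to the manager's StartNewMatch, with no actor filter or re-trigger guard.
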(event Collision|EventActorBeginOverlap
  (params (OtherActor :type Actor%20Object%20Reference))
  ;[0.15 0.15 0.15 0.5] Start Match
  (bind _sportdata (Variables|Default|GetSportData)
    (:then
      (Class|DebugFunctionLibrary|DebugPrint "Debug" (Utilities|String|ToString(Text) (Utilities|Text|FormatText "{Game} Started" (Utilities|String|EnumtoString (Variables|/Script/ProjectGrace.SportDataAsset|GetSportType _sportdata)))) "Info" (CallFunction|GetEnablePrintscreen) (CallFunction|GetEnableLog) 5.0 false "None")
      (Class|SportManager|StartNewMatch (Variables|Default|GetSportManager) (Variables|Default|GetSportData)))
    (:else)))

(event EventBeginPlay
  ;[0.15 0.15 0.15 0.5] Begin play
  (Utilities|FlowControl|Delay 0.2)
  (bind _returnvalue (Actor|GetActorOfClass "/Script/ProjectGrace.SportManager"))
  (Utilities|IsValid _returnvalue
    (:Is%20Valid
      (Variables|Default|SetSportManager _returnvalue))
    (:Is%20Not%20Valid
      (Class|DebugFunctionLibrary|DebugPrint "Sport" "Sport manager does not exist! Spawned one" "Warning" (CallFunction|GetEnablePrintscreen) (CallFunction|GetEnableLog) 5.0 false "None")
      (bind _returnvalue_2 (Game|SpawnActorfromClass "/Game/Sport/BP_SportManager.BP_SportManager_C" (Math|Transform|MakeTransform "0, 0, 0" "0, 0, 0" "1.000000,1.000000,1.000000") "Undefined" "MultiplyWithRoot" 0 0))
      (Variables|Default|SetSportManager _returnvalue_2))))

(fn ConstructionScript)