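; Gameplay ability that throws the current weapon's projectile from the character.
; On activation it listens for Throw and Fire gameplay events and calls Fire on the WeaponComponent; the Fire event ends the ability.
; The Throw event async-loads the weapon's projectile class and mesh, then spawns it at the "Bat" socket.
; Its velocity is the socket's world location plus a scaled eye-view forward vector.
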(event Ability|EventActivateAbility
  (Variables|Default|SetWeaponComp (Actor|GetComponentbyClass (Ability|GetAvatarActorfromActorInfo) "/Script/ProjectGrace.WeaponComponent"))
  (Ability|Tasks|WaitGameplayEvent "(TagName=\"Event.Combat.Weapon.Throw\")" 0
    (:then
      (Ability|Tasks|WaitGameplayEvent "(TagName=\"Event.Combat.Weapon.Fire\")" 0
        (:then
          (Class|WeaponComponent|Fire (Variables|Default|GetWeaponComp)))
        (:EventReceived
          (Ability|EndAbility))))
    (:EventReceived
      ;[0.15 0.15 0.15 0.5] Spawn the projectile
      (bind _class (Class|BPIWeapon|GetProjectileClass(Message) (Class|WeaponComponent|GetCurrentWeapon (Variables|Default|GetWeaponComp))))
      (Utilities|AsyncLoadClassAsset _class
        (:Completed
          (bind _mesh (Class|BPIWeapon|GetProjectileMesh(Message) (Class|WeaponComponent|GetCurrentWeapon (Variables|Default|GetWeaponComp))))
          (Utilities|AsyncLoadAsset _mesh
            (:Completed
              (Game|SpawnActorfromClass (Utilities|ResolveSoftReference _class) (Math|Transform|MakeTransform (Transformation|GetSocketLocation (Actor|GetComponentbyClass (Ability|GetAvatarActorfromActorInfo) "/Script/Engine.SkeletalMeshComponent") "Bat") "0, 0, 0" "1.000000,1.000000,1.000000") "AlwaysSpawn" "MultiplyWithRoot" (Ability|GetAvatarActorfromActorInfo) (Utilities|ResolveSoftReference _mesh) (CallFunction|GetVelocity) 0))))))))

(fn GetVelocity
  (return (+ (Transformation|GetSocketLocation (Actor|GetComponentbyClass (Ability|GetAvatarActorfromActorInfo) "/Script/Engine.SkeletalMeshComponent") "Bat") (* (Math|Vector|GetForwardVector (.OutRotation (Actor|GetActorEyesViewPoint (Ability|GetAvatarActorfromActorInfo)))) 8e+02))))