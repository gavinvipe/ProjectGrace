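; GA_Ragdoll is an event-triggered gameplay ability that temporarily puts the avatar into full ragdoll.
; It enables the avatar's RagdollComponent right after starting a wait for the ragdoll-enable gameplay event.
; That event applies a velocity impulse below a bone and plays a montage, both driven by the activation payload.
; Montage completion plus a short delay, or immediate interruption or cancellation, disables ragdoll and ends the ability.
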(event Ability|EventActivateAbilityFromEvent
  (params (EventData :type Gameplay%20Event%20Data%20Structure%20%28by%20ref%29))
  (bind _asobp_ability_payload (Utilities|Casting|CastToOBP_AbilityPayload (.optionalobject EventData)))
  (Variables|Default|SetAbilityPayload _asobp_ability_payload)
  (bind _output_get (Variables|Default|SetRagdollComp (Actor|GetComponentbyClass (Ability|GetAvatarActorfromActorInfo) "/Script/ProjectGrace.RagdollComponent")))
  (Variables|/Script/ProjectGrace.RagdollComponent|SetbEnableFullRagdoll _output_get true)
  (Ability|Tasks|WaitGameplayEvent "(TagName=\"Event.Ragdoll.Enable\")" 0
    (:then
      (Class|RagdollComponent|EnableRagdoll (Variables|Default|GetRagdollComp)))
    (:EventReceived
      (Class|SkeletalMeshComponent|AddImpulsetoAllBodiesBelow (Utilities|Struct|BreakGameplayAbilityActorInfo (Ability|GetActorInfo)) (Variables|/Game/GameplayAbilities/Payloads/OBP_AbilityPayload.OBP_AbilityPayload_C|GetMessageVector (Variables|Default|GetAbilityPayload)) (Variables|/Game/GameplayAbilities/Payloads/OBP_AbilityPayload.OBP_AbilityPayload_C|GetMessageName (Variables|Default|GetAbilityPayload)) true false)
      (|PlayMontageandWaitProxy "None" (Variables|/Game/GameplayAbilities/Payloads/OBP_AbilityPayload.OBP_AbilityPayload_C|GetMessageMontage (Variables|Default|GetAbilityPayload)) 1.0 "None" true 1.0 0.0 true
        (:OnCompleted
          (Ability|Tasks|WaitDelay 3.0
            (:OnFinish
              _)))
        (:OnInterrupted
          _)
        (:OnCancelled
          _))
      (Class|RagdollComponent|DisableRagdoll (Variables|Default|GetRagdollComp))
      (Ability|EndAbility))))