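; Gameplay ability that plays a character's hit reaction montage when activated from a gameplay event.
; It reads the montage from the event's OBP_AbilityPayload object, stopping without ending the ability if that cast fails.
; The ability ends when the montage completes, is interrupted or is cancelled.
; Disconnected leftover nodes hold an unused ragdoll reaction with a bone impulse and a timed end.
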(event Ability|EventActivateAbilityFromEvent
  (params (EventData :type Gameplay%20Event%20Data%20Structure%20%28by%20ref%29))
  (bind _asobp_ability_payload (Utilities|Casting|CastToOBP_AbilityPayload (.optionalobject EventData)))
  (Variables|Default|SetAbilityPayload _asobp_ability_payload)
  (|PlayMontageandWaitProxy "None" (Variables|/Game/GameplayAbilities/Payloads/OBP_AbilityPayload.OBP_AbilityPayload_C|GetMessageMontage (Variables|Default|GetAbilityPayload)) 1.0 "None" true 1.0 0.0 true
    (:OnCompleted
      _)
    (:OnInterrupted
      _)
    (:OnCancelled
      _))
  (Ability|EndAbility))