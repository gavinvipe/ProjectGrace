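; GA_Grind is a ride ability that puts the rider onto a grindable spline, ending at once if none is found.
; It disables ground alignment, switches to Flying, then moves the capsule to the grind point at grind speed while tilting the rideable mesh.
; IsGrinding is set after the capsule move; the EndSkill event ends the ability.
; A Jump event wait also starts, but its received event has no handler.
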(event Ability|EventActivateAbility
  (bind _output_get (Variables|Default|SetRideableComponent (Actor|GetComponentbyClass (Ability|GetAvatarActorfromActorInfo) "/Script/ProjectGrace.RideableComponent")))
  (Utilities|IsValid _output_get
    (:Is%20Valid
      (bind _ascharacter (Utilities|Casting|CastToCharacter (Ability|GetAvatarActorfromActorInfo)))
      ;[0.15 0.15 0.15 0.5] Get grind details
      (Variables|Default|SetAs%20Character _ascharacter)
      (bind _returnvalue (Class|RideableMovementComponent|CheckGrindable (Variables|/Script/ProjectGrace.RideableComponent|GetRideableMovementComponent (Variables|Default|GetRideableComponent))))
      (if (.bisgrindable _returnvalue)
        (Ability|Tasks|WaitGameplayEvent "(TagName=\"Event.Ride.Jump\")" 0
          (:then
            (Ability|Tasks|WaitGameplayEvent "(TagName=\"Event.Ride.EndSkill\")" 0
              (:then
                (Variables|/Script/ProjectGrace.RideableMovementComponent|SetbDisableGroundAlignment (Variables|/Script/ProjectGrace.RideableComponent|GetRideableMovementComponent (Variables|Default|GetRideableComponent)) true)
                (Pawn|Components|CharacterMovement|SetMovementMode (Variables|/Script/Engine.Character|GetCharacterMovement (Variables|Default|GetAs%20Character)) "MOVE_Flying" 0)
                (Utilities|FlowControl|Sequence
                  (:then_0
                    ;[0.15 0.15 0.15 0.5] Rotate Rideable Mesh
                    (Components|MoveComponentTo (Variables|/Script/ProjectGrace.Rideable|GetMesh (Variables|/Script/ProjectGrace.RideableComponent|GetCurrentRideable (Variables|Default|GetRideableComponent))) (Variables|/Script/Engine.SceneComponent|GetRelativeLocation (Variables|/Script/ProjectGrace.Rideable|GetMesh (Variables|/Script/ProjectGrace.RideableComponent|GetCurrentRideable (Variables|Default|GetRideableComponent)))) "20.000000,-30.000000,0.000000" false false (/ (Math|Vector|Distance(Vector) (+ (Spline|GetLocationatDistanceAlongSpline (.Spline (Utilities|Struct|BreakGrindable (Variables|/Script/ProjectGrace.RideableMovementComponent|GetGrindableDetails (Variables|/Script/ProjectGrace.RideableComponent|GetRideableMovementComponent (Variables|Default|GetRideableComponent))))) (.GrindPoint (Utilities|Struct|BreakGrindable (Variables|/Script/ProjectGrace.RideableMovementComponent|GetGrindableDetails (Variables|/Script/ProjectGrace.RideableComponent|GetRideableMovementComponent (Variables|Default|GetRideableComponent))))) "World") (Math|Vector|MakeVector 0.0 0.0 (Variables|/Script/Engine.CapsuleComponent|GetCapsuleHalfHeight (Variables|/Script/Engine.Character|GetCapsuleComponent (Variables|Default|GetAs%20Character)))) (Math|Vector|MakeVector 0.0 0.0 (.GrindOffset (Utilities|Struct|BreakGrindable (Variables|/Script/ProjectGrace.RideableMovementComponent|GetGrindableDetails (Variables|/Script/ProjectGrace.RideableComponent|GetRideableMovementComponent (Variables|Default|GetRideableComponent))))))) (Transformation|GetWorldLocation (Variables|/Script/Engine.Character|GetCapsuleComponent (Variables|Default|GetAs%20Character)))) (Variables|/Script/ProjectGrace.RideableMovementComponent|GetGrindSpeed (Variables|/Script/ProjectGrace.RideableComponent|GetRideableMovementComponent (Variables|Default|GetRideableComponent)))) false))
                  (:then_1
                    ;[0.15 0.15 0.15 0.5] Move capsule component over time on grind
                    (Components|MoveComponentTo (Variables|/Script/Engine.Character|GetCapsuleComponent (Variables|Default|GetAs%20Character)) (+ (Spline|GetLocationatDistanceAlongSpline (.Spline (Utilities|Struct|BreakGrindable (Variables|/Script/ProjectGrace.RideableMovementComponent|GetGrindableDetails (Variables|/Script/ProjectGrace.RideableComponent|GetRideableMovementComponent (Variables|Default|GetRideableComponent))))) (.GrindPoint (Utilities|Struct|BreakGrindable (Variables|/Script/ProjectGrace.RideableMovementComponent|GetGrindableDetails (Variables|/Script/ProjectGrace.RideableComponent|GetRideableMovementComponent (Variables|Default|GetRideableComponent))))) "World") (Math|Vector|MakeVector 0.0 0.0 (Variables|/Script/Engine.CapsuleComponent|GetCapsuleHalfHeight (Variables|/Script/Engine.Character|GetCapsuleComponent (Variables|Default|GetAs%20Character)))) (Math|Vector|MakeVector 0.0 0.0 (.GrindOffset (Utilities|Struct|BreakGrindable (Variables|/Script/ProjectGrace.RideableMovementComponent|GetGrindableDetails (Variables|/Script/ProjectGrace.RideableComponent|GetRideableMovementComponent (Variables|Default|GetRideableComponent))))))) (Math|Rotator|MakeRotator 0.0 0.0 (+ (.yaw (Spline|GetRotationatDistanceAlongSpline (.Spline (Utilities|Struct|BreakGrindable (Variables|/Script/ProjectGrace.RideableMovementComponent|GetGrindableDetails (Variables|/Script/ProjectGrace.RideableComponent|GetRideableMovementComponent (Variables|Default|GetRideableComponent))))) (.GrindPoint (Utilities|Struct|BreakGrindable (Variables|/Script/ProjectGrace.RideableMovementComponent|GetGrindableDetails (Variables|/Script/ProjectGrace.RideableComponent|GetRideableMovementComponent (Variables|Default|GetRideableComponent))))) "World")) (Math|Float|SelectFloat 0.0 1.8e+02 (> (.GrindDirection (Utilities|Struct|BreakGrindable (Variables|/Script/ProjectGrace.RideableMovementComponent|GetGrindableDetails (Variables|/Script/ProjectGrace.RideableComponent|GetRideableMovementComponent (Variables|Default|GetRideableComponent))))) 0.0)))) false false (/ (Math|Vector|Distance(Vector) (+ (Spline|GetLocationatDistanceAlongSpline (.Spline (Utilities|Struct|BreakGrindable (Variables|/Script/ProjectGrace.RideableMovementComponent|GetGrindableDetails (Variables|/Script/ProjectGrace.RideableComponent|GetRideableMovementComponent (Variables|Default|GetRideableComponent))))) (.GrindPoint (Utilities|Struct|BreakGrindable (Variables|/Script/ProjectGrace.RideableMovementComponent|GetGrindableDetails (Variables|/Script/ProjectGrace.RideableComponent|GetRideableMovementComponent (Variables|Default|GetRideableComponent))))) "World") (Math|Vector|MakeVector 0.0 0.0 (Variables|/Script/Engine.CapsuleComponent|GetCapsuleHalfHeight (Variables|/Script/Engine.Character|GetCapsuleComponent (Variables|Default|GetAs%20Character)))) (Math|Vector|MakeVector 0.0 0.0 (.GrindOffset (Utilities|Struct|BreakGrindable (Variables|/Script/ProjectGrace.RideableMovementComponent|GetGrindableDetails (Variables|/Script/ProjectGrace.RideableComponent|GetRideableMovementComponent (Variables|Default|GetRideableComponent))))))) (Transformation|GetWorldLocation (Variables|/Script/Engine.Character|GetCapsuleComponent (Variables|Default|GetAs%20Character)))) (Variables|/Script/ProjectGrace.RideableMovementComponent|GetGrindSpeed (Variables|/Script/ProjectGrace.RideableComponent|GetRideableMovementComponent (Variables|Default|GetRideableComponent)))) false)
                    (Variables|/Script/ProjectGrace.RideableMovementComponent|SetbIsGrinding (Variables|/Script/ProjectGrace.RideableComponent|GetRideableMovementComponent (Variables|Default|GetRideableComponent)) true))))
              (:EventReceived
                (Ability|EndAbility))))
          (:EventReceived))
        (else
          (Ability|EndAbility))))
    (:Is%20Not%20Valid
      (Ability|EndAbility))))