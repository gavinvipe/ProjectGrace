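; GA_KickFlip is a gameplay ability that performs a kickflip jump on the avatar's current rideable.
; On activation it registers gameplay event listeners, then immediately calls Jump on the rideable's movement component.
; Event.Ride.Jump makes the rider Character jump.
; Event.Ride.EndSkill has two listeners: one plays a non-looping animation on the rideable mesh, the other stops the rider's jump and ends the ability.
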(event Ability|EventActivateAbility
  (bind _currentrideable (Variables|/Script/ProjectGrace.RideableComponent|GetCurrentRideable (Actor|GetComponentbyClass (Ability|GetAvatarActorfromActorInfo) "/Script/ProjectGrace.RideableComponent"))
    (:then
      (Variables|Default|SetCurrent%20Rideable _currentrideable)
      (Ability|Tasks|WaitGameplayEvent "(TagName=\"Event.Ride.EndSkill\")" 0
        (:then
          (bind _ascharacter (Utilities|Casting|CastToCharacter (Ability|GetAvatarActorfromActorInfo)))
          (Variables|Default|SetAs%20Character _ascharacter)
          (Ability|Tasks|WaitGameplayEvent "(TagName=\"Event.Ride.Jump\")" 0
            (:then
              (Ability|Tasks|WaitGameplayEvent "(TagName=\"Event.Ride.EndSkill\")" 0
                (:then
                  (Class|RideableMovementComponent|Jump (Actor|GetComponentbyClass (Variables|Default|GetCurrent%20Rideable) "/Script/ProjectGrace.RideableMovementComponent")))
                (:EventReceived
                  (Character|StopJumping (Variables|Default|GetAs%20Character))
                  (Ability|EndAbility))))
            (:EventReceived
              (Character|Jump (Variables|Default|GetAs%20Character)))))
        (:EventReceived
          (Components|Animation|PlayAnimation (Variables|/Script/ProjectGrace.Rideable|GetMesh (Variables|Default|GetCurrent%20Rideable)) 0 false))))
    (:else)))