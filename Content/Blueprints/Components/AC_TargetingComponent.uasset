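; Actor component for assisted-aim lock-on that steers player control rotation toward a living target.
; ScanTargets runs async Targeting System presets for partial or full assist, with a short cooldown, and FIndTarget picks the candidate with least sideways camera offset.
; UpdateLock interpolates toward the target's interface-provided lock point, rescanning when it is invalid, dead or out of range.
; ChangeTarget reselects excluding the current target under full assist, otherwise clears it.
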(event EventChangeTarget
  ;[0.15 0.15 0.15 0.5] Change target
  (if (Utilities|Enum|Equal(Enum) (Variables|Default|GetAssitedAim) "Full")
    (Utilities|Array|RemoveItem (Variables|Default|GetTargets) (Variables|Default|GetCurrentTarget))
    (Variables|Default|SetPrevious%20Target (Variables|Default|GetCurrentTarget))
    (Targeting|FIndTarget)
    (Utilities|Array|AddUnique (Variables|Default|GetTargets) (Variables|Default|GetPrevious%20Target))
    (else
      (Variables|Default|SetCurrentTarget 0))))

(event EventScanTargets
  ;[0.15 0.15 0.15 0.5] Scan Targets
  (if (Utilities|Enum|NotEqual(Enum) (Variables|Default|GetAssitedAim) "Free")
    (Variables|Target|GetIsScanning
      (:then)
      (:else
        (Variables|Target|SetIsScanning true)
        (bind _targetinghandle (|PerformTargetingRequest (Components|GetOwner) (Utilities|Select :Index (Variables|Default|GetAssitedAim) :Free 0 :Partial "/Game/Blueprints/Data/TargetPreset/TP_PartialAim.TP_PartialAim" :Full "/Game/Blueprints/Data/TargetPreset/TP_FullAim.TP_FullAim") true)
          (:Targeted
            (Variables|Default|SetTargets (Class|TargetingSubsystem|GetTargetingResultsActors (GameInstanceSubsystems|GetTargetingSubsystem) _targetinghandle))
            (Targeting|FIndTarget)
            (Utilities|FlowControl|Delay 0.2)
            (Variables|Target|SetIsScanning false)))))))

(fn UpdateLock
  (if (Utilities|Enum|NotEqual(Enum) (Variables|Default|GetAssitedAim) "Free")
    (bind _currenttarget (Variables|Default|GetCurrentTarget)
      (:then
        (if (> (Math|Vector|Distance(Vector) (Transformation|GetActorLocation _currenttarget) (Transformation|GetActorLocation (Components|GetOwner))) 1e+03)
          (Class|TargetingComponent|ScanTargets :!label _label)
          (else
            (bind _return (Class|BPICharacter|GetIsDead(Message) (Variables|Default|GetCurrentTarget)))
            (if _return
              (goto _label)
              (else
                (bind _location (Class|BPICharacter|GetLockonLocation(Message) (Variables|Default|GetCurrentTarget)))
                (Pawn|SetControlRotation (Game|GetPlayerController 0) (Math|Interpolation|RInterpTo (Pawn|GetControlRotation (Game|GetPlayerController 0) :!class /Script/Engine.Controller) (Math|Rotator|FindLookatRotation (Camera|GetCameraLocation (Game|GetPlayerCameraManager 0)) _location) (Utilities|Time|GetWorldDeltaSeconds) (Variables|Target|GetLockOnSpeed))))))))
      (:else
        (Class|TargetingComponent|ScanTargets)))))

(fn FIndTarget
  (bind _returnvalue (Game|GetPlayerCameraManager 0))
  (for _array_element (Variables|Default|GetTargets)
    (bind _return (Class|BPICharacter|GetIsDead(Message) _array_element))
    (if _return
      (Utilities|Array|RemoveItem (Variables|Default|GetTargets) _array_element)
      (else
        (bind _location (Class|BPICharacter|GetLockonLocation(Message) _array_element))
        (if (< (Math|Float|Absolute(Float) (Math|Vector|DotProduct (- _location (Camera|GetCameraLocation _returnvalue)) (Math|Vector|GetRightVector (Camera|GetCameraRotation _returnvalue)))) (LocalVariables|GetClosestDistance))
          (LocalVariables|SetClosestDistance (Math|Float|Absolute(Float) (Math|Vector|DotProduct (- _location (Camera|GetCameraLocation _returnvalue)) (Math|Vector|GetRightVector (Camera|GetCameraRotation _returnvalue)))))
          (LocalVariables|SetTempTarget _array_element)))))
  (Variables|Default|SetCurrentTarget (LocalVariables|GetTempTarget))
  (return))

(fn TargetDebug
  (for _array_element (Variables|Default|GetTargets)
    (Rendering|Debug|DrawDebugBox (Transformation|GetActorLocation _array_element) "50.000000,50.000000,50.000000" "(R=0.253796,G=0.848946,B=1.000000,A=1.000000)" "0, 0, 0" 5.0 1.0)))