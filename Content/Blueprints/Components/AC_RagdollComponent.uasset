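; Actor component that switches its owning character in and out of physics ragdoll, with a debug key toggle.
; Enabling drops capsule collision, simulates from the pelvis and sets Physics Control limb controls.
; Each tick scales joint strength by velocity, caps falling acceleration and moves the actor to the pelvis using a floor trace.
; Disabling destroys those controls, snapshots the pose, then plays a Chooser-picked get-up montage or resumes falling with ragdoll velocity.
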(event EventDisableRagdoll
  (bind _mesh (Variables|Default|GetMesh))
  (bind _charactermovement (Variables|Default|GetCharacterMovement))
  ;[0.15 0.15 0.15 0.5] Disable ragdoll
  (Variables|Default|GetbIsRagdolling
    (:then
      (Utilities|FlowControl|Sequence
        (:then_0
          ;;[1 1 1] Update the Actor location to follow the ragdoll.
          (Class|PhysicsControlComponent|DestroyAllControlsandBodyModifiers (Variables|Default|GetPhysicsControl)))
        (:then_1
          ;;[1 1 1] Step 1: Save a snapshot of the current Ragdoll Pose for use in AnimGraph to blend out of the ragdoll
          (Class|AnimInstance|SavePoseSnapshot (Components|SkeletalMesh|GetAnimInstance (Variables|Default|GetMesh)) "RagdollPose"))
        (:then_2
          ;;[1 1 1] Step 2: If the ragdoll is on the ground, set the movement mode to walking and play a Get Up animation. If not, set the movement mode to falling and update teh character movement velocity to match the last ragdoll velocity.
          (if (Variables|Ragdoll|GetRagdollOnGround)
            (Pawn|Components|CharacterMovement|SetMovementMode _charactermovement "MOVE_Walking" 0)
            (bind _output (Utilities|GetUpAnimation)
              (:Completed
                (Animation|Montage|MontagePlay (Components|SkeletalMesh|GetAnimInstance (Variables|Default|GetMesh)) _output 1.0 "MontageLength" 0.0 true)))
            (else
              (Pawn|Components|CharacterMovement|SetMovementMode _charactermovement "MOVE_Falling" 0)
              (Variables|/Script/Engine.MovementComponent|SetVelocity (Variables|Default|GetCharacterMovement) (Variables|Ragdoll|GetLastRagdollVelocity)))))
        (:then_3
          ;;[1 1 1] Step 3: Re-Enable capsule collision, and disable physics simulation on the mesh.
          (Utilities|FlowControl|Delay 0.3)
          (Collision|SetCollisionEnabled (Variables|Default|GetCapsuleComponent) "QueryAndPhysics")
          (Collision|SetCollisionObjectType _mesh "ECC_GameTraceChannel1")
          (Collision|SetCollisionEnabled _mesh "QueryOnly")
          (Class|SkeletalMeshComponent|SetAllBodiesSimulatePhysics _mesh false))
        (:then_4
          (Variables|Default|SetbIsRagdolling false))))
    (:else)))

(event EventBeginPlay
  (bind _returnvalue (Components|GetOwner))
  ;[0.15 0.15 0.15 0.5] Begin play
  (Variables|Default|SetMesh (Actor|GetComponentbyClass _returnvalue "/Script/Engine.SkeletalMeshComponent"))
  (Variables|Default|SetCharacterMovement (Actor|GetComponentbyClass _returnvalue "/Script/Engine.CharacterMovementComponent"))
  (Variables|Default|SetCapsuleComponent (Actor|GetComponentbyClass _returnvalue "/Script/Engine.CapsuleComponent"))
  (bind _output_get (Variables|Default|SetPhysicsControl (Actor|GetComponentbyClass _returnvalue "/Script/PhysicsControl.PhysicsControlComponent")))
  (Class|PhysicsControlComponent|CreateControlsandBodyModifiersfromLimbBones _output_get (Variables|Default|GetMesh) (Variables|Ragdoll|Physics|GetLimb%20Setup%20Data) (Variables|Ragdoll|Physics|GetWorld%20Space%20Control%20Data) (Variables|Ragdoll|Physics|GetParent%20Space%20Control%20Data) (Variables|Ragdoll|Physics|GetBody%20Modifier%20Data) 0 "None"))

(event EventTick
  (params (DeltaSeconds :type Float%20%28single-precision%29))
  ;[0.15 0.15 0.15 0.5] Tick
  (if (Variables|Default|GetbIsRagdolling)
    (CallFunction|UpdateRagdoll)))

(event Input|KeyboardEvents|DebugKeyR
  (params (Key :type Key%20Structure) (ActionValue :type Input%20Action%20Value%20Structure))
  (:Pressed
    (Utilities|FlowControl|FlipFlop
      (:A
        (CallFunction|EnableRagdoll))
      (:B
        (Class|RagdollComponent|DisableRagdoll)))))

(fn EnableRagdoll
  (bind _mesh (Variables|Default|GetMesh))
  (if (not (Variables|Default|GetbIsRagdolling))
    (Utilities|FlowControl|Sequence
      (:then_0
        ;[1 1 1] Step 1: Stop any active montages - Done first to stop Traversal Montages
        (Animation|Montage|MontageStop (Components|SkeletalMesh|GetAnimInstance (Variables|Default|GetMesh)) 0.0 0))
      (:then_1
        ;[1 1 1] Step 2: Clear the Character Movement Mode and set the Ragdoll Flag
        (Pawn|Components|CharacterMovement|SetMovementMode (Variables|Default|GetCharacterMovement) "MOVE_None" 0)
        (Variables|Default|SetbIsRagdolling true))
      (:then_2
        ;[1 1 1] Step 3: Disable capsule collision and enable mesh physics simulation starting from the pelvis.
        (Collision|SetCollisionEnabled (Variables|Default|GetCapsuleComponent) "NoCollision")
        (Collision|SetCollisionObjectType _mesh "ECC_PhysicsBody")
        (Collision|SetCollisionEnabled _mesh "QueryAndPhysics")
        (Class|SkeletalMeshComponent|SetAllBodiesBelowSimulatePhysics _mesh (Utilities|Name|MakeLiteralName "pelvis") true true))
      (:then_3
        ;[0.15 0.15 0.15 0.5] Set controls
        (Class|PhysicsControlComponent|SetControlsinSetEnabled (Variables|Default|GetPhysicsControl) "All" (not (Variables|Default|GetbEnableFullRagdoll))))
      (:then_4
        ;[0.15 0.15 0.15 0.5] End enabled ragdoll
        (Ability|SendGameplayEventtoActor (Components|GetOwner) "(TagName=\"Event.Ragdoll.Enable\")")))))

(fn UpdateRagdoll
  (Utilities|FlowControl|Sequence
    (:then_0
      ;[1 1 1] Set the Last Ragdoll Velocity.
      (bind _returnvalue (Physics|GetPhysicsLinearVelocity (Variables|Default|GetMesh) "root"))
      (Variables|Ragdoll|SetLastRagdollVelocity _returnvalue))
    (:then_1
      ;[1 1 1] Use the Ragdoll Velocity to scale the ragdoll's joint strength for physical animation.
      (Class|SkeletalMeshComponent|SetAllMotorsAngularDriveParams (Variables|Default|GetMesh) (Math|Float|MapRangeClamped (Math|Vector|VectorLength (Variables|Ragdoll|GetLastRagdollVelocity)) 0.0 1e+03 0.0 2.5e+04) 0.0 0.0 false))
    (:then_2
      ;[1 1 1] Disable Gravity if falling faster than -4000 to prevent continual acceleration. This also prevents the ragdoll from going through the floor.
      (Physics|SetEnableGravity (Variables|Default|GetMesh) (> (.z (Variables|Ragdoll|GetLastRagdollVelocity)) -4e+03)))
    (:then_3
      (Ragdoll|SetActorLocationDuringRagdoll))))

(fn SetActorLocationDuringRagdoll
  (bind _mesh (Variables|Default|GetMesh))
  (bind _returnvalue (Transformation|GetSocketRotation _mesh "pelvis"))
  (Utilities|FlowControl|Sequence
    (:then_0
      ;[1 1 1] Set the pelvis as the target location.
      (LocalVariables|SetTargetRagdollLocation (Transformation|GetSocketLocation (Variables|Default|GetMesh) "pelvis")))
    (:then_1
      ;[1 1 1] Determine wether the ragdoll is facing up or down and set the target rotation accordingly.
      (bind _output_get (Variables|Ragdoll|SetRagdollFaceUp (< (.roll _returnvalue) 0.0)))
      (LocalVariables|SetTargetRagdollRotation (Math|Rotator|MakeRotator 0.0 0.0 (select _output_get (- (.yaw _returnvalue) 1.8e+02) (.yaw _returnvalue)))))
    (:then_2
      ;[1 1 1] Trace downward from the target location to offset the target location, preventing the lower half of the capsule from going through the floor when the ragdoll is laying on the ground.
      (bind _outhit (Collision|LineTraceByChannel (LocalVariables|GetTargetRagdollLocation) (Math|Vector|MakeVector (.X (Math|Vector|BreakVector (LocalVariables|GetTargetRagdollLocation))) (.Y (Math|Vector|BreakVector (LocalVariables|GetTargetRagdollLocation))) (- (.Z (Math|Vector|BreakVector (LocalVariables|GetTargetRagdollLocation))) (Components|Capsule|GetScaledCapsuleHalfHeight (Variables|Default|GetCapsuleComponent)))) "TraceTypeQuery1" false 0 "None"))
      (bind _output_get_2 (Variables|Ragdoll|SetRagdollOnGround (.bblockinghit _outhit)))
      (if _output_get_2
        (Ragdoll|SetActorLocationandRotation(UpdateTarget) (Math|Vector|MakeVector (.X (Math|Vector|BreakVector (LocalVariables|GetTargetRagdollLocation))) (.Y (Math|Vector|BreakVector (LocalVariables|GetTargetRagdollLocation))) (+ (.Z (Math|Vector|BreakVector (LocalVariables|GetTargetRagdollLocation))) (- (Components|Capsule|GetScaledCapsuleHalfHeight (Variables|Default|GetCapsuleComponent)) (Math|Float|Absolute(Float) (- (.z (.impactpoint _outhit)) (.z (.tracestart _outhit))))) 2.0)) (LocalVariables|GetTargetRagdollRotation) false false)
        (else
          (Ragdoll|SetActorLocationandRotation(UpdateTarget) (LocalVariables|GetTargetRagdollLocation) (LocalVariables|GetTargetRagdollRotation) false false))))))

(fn SetActorLocationandRotation(UpdateTarget)
  (params (NewLocation :type Vector) (NewRotation :type Rotator) (bSweep :type Boolean) (bTeleport :type Boolean))
  (bind _output_get (Variables|Ragdoll|SetRagdollTargetRotation NewRotation))
  (bind (_sweephitresult _returnvalue) (Transformation|SetActorLocationAndRotation (Components|GetOwner) NewLocation _output_get bSweep bTeleport))
  (return _sweephitresult _returnvalue))