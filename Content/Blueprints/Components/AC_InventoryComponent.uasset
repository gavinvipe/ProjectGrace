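; Inventory actor component that stores items in a map keyed by ItemID, with a data asset and stack count per entry.
; Adding increments an existing stack or creates an entry from DT_Items while under InventorySize; removing decrements or deletes it.
; Both operations return whether a stack or the inventory changed, and adding can report Full.
; The stack-limit check compares the table's StackSize with itself plus one, ignoring the held count.
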(event EventBeginPlay
  ;[0.15 0.15 0.15 0.5] Begin play
  (Variables|Default|SetOwner (Components|GetOwner)))

(fn GetStackSize
  (params (ItemID :type Name :default "None"))
  (bind _returnvalue (Utilities|GetDataTableRow "/Game/Blueprints/Data/DataTables/DT_Items.DT_Items" ItemID)
    (:then
      (return (.StackSize (Utilities|Struct|BreakInventoryItem _returnvalue))))))

(fn AddtoInventory
  (params (ItemID :type Name :default "None"))
  (bind _items (Variables|Default|GetItems))
  (bind _value (Utilities|Map|Find _items ItemID))
  (bind (_dataasset _stacksize) (Utilities|Struct|BreakInventoryItem _value))
  (if (.ReturnValue (Utilities|Map|Find (Variables|Default|GetItems) ItemID))
    (bind _returnvalue (Utilities|GetDataTableRow "/Game/Blueprints/Data/DataTables/DT_Items.DT_Items" ItemID)
      (:then
        (if (< (CallFunction|GetStackSize ItemID) (+ (.StackSize (Utilities|Struct|BreakInventoryItem _returnvalue)) 1))
          (Utilities|Map|Add _items ItemID (Utilities|Struct|MakeInventoryItem _dataasset (+ _stacksize 1)))
          (return "Stack")
          (else
            (return "Full")))))
    (elif (< (Utilities|Map|Length (Variables|Default|GetItems)) (Variables|Default|GetInventorySize))
      (bind _returnvalue_2 (Utilities|GetDataTableRow "/Game/Blueprints/Data/DataTables/DT_Items.DT_Items" ItemID)
        (:then
          (Utilities|Map|Add (Variables|Default|GetItems) ItemID (Utilities|Struct|MakeInventoryItem (.DataAsset (Utilities|Struct|BreakInventoryItem _returnvalue_2)) 1))
          (return "Inventory")))
      (else
        (return "Full")))))

(fn RemovefromInventory
  (params (ItemID :type Name :default "None"))
  (bind _items (Variables|Default|GetItems))
  (bind _items_2 (Variables|Default|GetItems))
  (bind (_value _returnvalue) (Utilities|Map|Find _items ItemID))
  (bind _value_2 (Utilities|Map|Find _items_2 ItemID))
  (bind (_dataasset _stacksize) (Utilities|Struct|BreakInventoryItem _value_2))
  (if _returnvalue
    (if (> (.StackSize (Utilities|Struct|BreakInventoryItem _value)) 1)
      (Utilities|Map|Add (Variables|Default|GetItems) ItemID (Utilities|Struct|MakeInventoryItem _dataasset (- _stacksize 1)))
      (return "Stack")
      (else
        (Utilities|Map|Remove (Variables|Default|GetItems) ItemID)
        (return "Inventory")))))

(fn GetItemDetails
  (params (Item :type Name :default "None"))
  (bind _items (Variables|Default|GetItems))
  (bind (_value _returnvalue) (Utilities|Map|Find _items Item))
  (return _returnvalue _value))