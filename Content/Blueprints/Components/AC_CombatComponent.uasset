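; Melee combat component for player and AI characters, handling light/heavy attacks, combos, blocking and timed parries.
; Attack and parry inputs are time-buffered, then Chooser tables pick async-loaded montages, motion-warped toward nearby targets from the targeting component.
; Hits apply fixed GAS damage, send hit-reaction events, fire gameplay cues and report AI damage sense events.
; Non-AI owners also scan for targets before attacking and get brief global time-dilation hit-stop.
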(event EventPerformHeavyhtAttack
  ;[0.15 0.15 0.15 0.5] Heavy Attack
  (Variables|Default|SetbIsLightAttack false)
  (Variables|Default|SetbIsHeavyAttack true)
  (Combat|Attack))

(event EventPlayCombatAnim
  ;[0.15 0.15 0.15 0.5] Play selected anim
  (bind _targetcomponent (Variables|Default|GetTargetComponent)
    (:then
      (Utilities|IsValid (AI|GetAIController (Components|GetOwner))
        (:Is%20Valid
          _)
        (:Is%20Not%20Valid
          (Class|TargetingComponent|ScanTargets _targetcomponent)
          (Utilities|FlowControl|Delay 0.2)))
      (Utilities|IsValid (Class|TargetingComponent|GetCurrentTarget _targetcomponent)
        (:Is%20Valid
          (if (< (Transformation|GetDistanceTo (Class|TargetingComponent|GetCurrentTarget _targetcomponent) (Components|GetOwner)) 4e+02)
            (Class|MotionWarpingComponent|AddorUpdateWarpTargetfromLocationandRotation (Variables|Default|GetMotionWarping) "Combat Move" (.Location (CallFunction|GetWarpLocationandRotation (Class|TargetingComponent|GetCurrentTarget _targetcomponent))) (.Rotation (CallFunction|GetWarpLocationandRotation (Class|TargetingComponent|GetCurrentTarget _targetcomponent))))))))
    (:else
      _))
  (bind _montage (Utilities|GetCombatAnim)
    (:Completed
      (Animation|Montage|PlayMontage (Variables|Default|GetMeshComp) _montage
        (:OnCompleted
          _)
        (:OnInterrupted
          _))
      (Variables|Default|SetCombatState "None")
      (Variables|Default|SetbIsAttacking false)
      (Variables|Default|SetbIsParrying false)
      (Variables|Default|SetbIsCombo false)
      (Class|CombatComponent|CheckCachedAttackInput)
      (Class|MotionWarpingComponent|RemoveWarpTarget (Variables|Default|GetMotionWarping) "Combat Move"))))

(event EventAttemptParry
  ;[0.15 0.15 0.15 0.5] Attempt Parry
  (if (Variables|Default|GetbIsParryWindowOpened)
    (Variables|Default|SetbIsParrying true)
    (Variables|Default|SetCombatState "Parrying")
    (Class|CombatComponent|PlayCombatAnim)
    (else
      (Variables|Default|SetCachedParryInputTime (Utilities|Time|GetTimeSeconds)))))

(event EventPerformLightAttack
  ;[0.15 0.15 0.15 0.5] Light Attack
  (Variables|Default|SetbIsHeavyAttack false)
  (Variables|Default|SetbIsLightAttack true)
  (Combat|Attack))

(event EventBeginPlay
  ;[0.15 0.15 0.15 0.5] Beginplay
  (Variables|Default|SetOwner (Components|GetOwner))
  (Variables|Default|SetMotionWarping (Actor|GetComponentbyClass (Variables|Default|GetOwner) "/Script/MotionWarping.MotionWarpingComponent"))
  (Variables|Default|SetMeshComp (Actor|GetComponentbyClass (Variables|Default|GetOwner) "/Script/Engine.SkeletalMeshComponent"))
  (Variables|Default|SetTargetComponent (Actor|GetComponentbyClass (Variables|Default|GetOwner) "/Script/ProjectGrace.TargetingComponent"))
  (Utilities|IsValid (AI|GetAIController (Variables|Default|GetOwner))))

(event EventBlock
  (params (bShouldBlock :type Boolean))
  ;[0.15 0.15 0.15 0.5] Block
  (if bShouldBlock
    (Variables|Default|SetbIsBlocking true)
    (Variables|Default|SetCombatState "Blocking")
    (else
      (Variables|Default|SetbIsBlocking false)
      (Variables|Default|SetCombatState "None"))))

(event EventCheckCachedAttackInput
  (bind _owner (Variables|Default|GetOwner))
  ;[0.15 0.15 0.15 0.5] Check input cache for valid attack
  (if (<= (- (Utilities|Time|GetTimeSeconds) (Variables|Default|GetCachedAttackInputTime)) 1.0)
    (Variables|Default|SetCachedAttackInputTime 0.0)
    (Combat|Attack)
    (else
      (Ability|SendGameplayEventtoActor _owner "(TagName=\"Event.Combat.Attack\")")
      (Ability|SendGameplayEventtoActor _owner "(TagName=\"Event.Combat.Parry\")"))))

(event EventApplyEffect
  ;[0.15 0.15 0.15 0.5] Apply Gameplay Effects
  (for _array_element (Variables|Default|GetHitResults)
    (Utilities|IsValid (Ability|GetAbilitySystemComponent (.HitActor (Collision|BreakHitResult _array_element)))
      (:Is%20Valid
        (if (not (Utilities|Array|ContainsItem (Variables|Default|GetHitActors) (.HitActor (Collision|BreakHitResult _array_element))))
          (Utilities|Array|AddUnique (Variables|Default|GetHitActors) (.HitActor (Collision|BreakHitResult _array_element)))
          (bind _montage (Utilities|GetReactionAnim)
            (:Completed
              (CallFunction|ActivateHitReaction _array_element _montage)
              (bind _returnvalue (Ability|GameplayEffect|AssignTagSetbyCallerMagnitude (GameplayEffects|MakeOutgoingSpec :self (Ability|GetAbilitySystemComponent (.HitActor (Collision|BreakHitResult _array_element))) :GameplayEffectClass "/Game/GameplayAbilities/Effects/GE_InstantDamage.GE_InstantDamage_C") "(TagName=\"Data.Damage.Instant\")" -15.0))
              (GameplayEffects|ApplyGameplayEffectSpecToSelf (Ability|GetAbilitySystemComponent (.HitActor (Collision|BreakHitResult _array_element))) _returnvalue)
              (GameplayCue|ExecuteGameplayCueOnActor(Burst) (.HitActor (Collision|BreakHitResult _array_element)) "(TagName=\"GameplayCue.Hit.LightAttack\")" (GameplayCue|MakeGameplayCueParametersfromHitResult _array_element))
              (Class|AISenseDamage|ReportDamageEvent (.HitActor (Collision|BreakHitResult _array_element)) (Components|GetOwner) 0.0 (Transformation|GetActorLocation (.HitActor (Collision|BreakHitResult _array_element))) (.ImpactPoint (Collision|BreakHitResult _array_element)) "Combat")))))))
  (Utilities|IsValid (AI|GetAIController (Components|GetOwner))
    (:Is%20Not%20Valid
      (Utilities|Time|SetGlobalTimeDilation 0.1)
      (Utilities|FlowControl|Delay 0.05)
      (Utilities|Time|SetGlobalTimeDilation 1.0))))

(event EventClearHitActors
  ;[0.15 0.15 0.15 0.5] Clear hit actors
  (Utilities|Array|Clear (Variables|Default|GetHitActors)))

(event EventParryWindow
  (params (bOpenWindow :type Boolean))
  ;[0.15 0.15 0.15 0.5] Parry window
  (bind _output_get (Variables|Default|SetbIsParryWindowOpened bOpenWindow))
  (if _output_get
    (if (not (Variables|Default|GetbIsParrying))
      (if (<= (- (Utilities|Time|GetTimeSeconds) (Variables|Default|GetCachedParryInputTime)) 2.0)
        (Variables|Default|SetCachedParryInputTime 0.0)
        (Class|CombatComponent|AttemptParry)))))

(fn Attack
  (Variables|Default|GetbCanAttack
    (:then
      (Variables|Default|GetbIsAttacking
        (:then
          ;[0.15 0.15 0.15 0.5] Cache attack
          (Variables|Default|SetCachedAttackInputTime (Utilities|Time|GetTimeSeconds)))
        (:else
          (Variables|Default|SetbIsAttacking true)
          (Variables|Default|SetCombatState "Attacking")
          (Variables|Default|SetComboCount 0)
          (Class|CombatComponent|PlayCombatAnim))))
    (:else)))

(fn GetWarpLocationandRotation
  (params (Target :type Actor%20Object%20Reference))
  (return (+ (* (Math|Vector|Normalize (- (Transformation|GetActorLocation (Variables|Default|GetOwner)) (Transformation|GetActorLocation Target))) 5e+01) (Transformation|GetActorLocation Target)) (Math|Rotator|FindLookatRotation (Transformation|GetActorLocation (Variables|Default|GetOwner)) (Transformation|GetActorLocation Target))))

(fn ActivateHitReaction
  (params (HitResult :type Hit%20Result%20Structure%20%28by%20ref%29) (Montage :type Anim%20Montage%20Object%20Reference))
  (bind (_bblockinghit _binitialoverlap _time _distance _location _impactpoint _normal _impactnormal _physmat _hitactor _hitcomponent _hitbonename) (Collision|BreakHitResult HitResult))
  (bind _returnvalue (Game|ConstructObjectfromClass "/Game/GameplayAbilities/Payloads/OBP_AbilityPayload.OBP_AbilityPayload_C"))
  (bind _output_get (LocalVariables|SetAbilityPayload _returnvalue))
  (Variables|/Game/GameplayAbilities/Payloads/OBP_AbilityPayload.OBP_AbilityPayload_C|SetMessageVector _output_get (* (Math|Vector|GetUnitDirection(Vector) (Transformation|GetActorLocation (Components|GetOwner)) _impactpoint) 2e+03))
  (Variables|/Game/GameplayAbilities/Payloads/OBP_AbilityPayload.OBP_AbilityPayload_C|SetMessageName (LocalVariables|GetAbilityPayload) _hitbonename)
  (Ability|SendGameplayEventtoActor _hitactor "(TagName=\"Event.HitReaction\")" (Utilities|Struct|MakeGameplayEventData "(TagName=\"\")" 0 0 (LocalVariables|GetAbilityPayload))))

(fn CheckCombo
  (if (<= (- (Utilities|Time|GetTimeSeconds) (Variables|Default|GetCachedAttackInputTime)) 1.0)
    (Variables|Default|SetbIsCombo true)
    (Variables|Default|SetCachedAttackInputTime 0.0)
    (Math|Integer|IncrementInt (Variables|Default|GetComboCount)
      (:%20%20
        (return true)))
    (else
      (return false))))

(fn CheckforParryActors
  (bind _bonename (Variables|Default|GetBoneName))
  (bind _meshcomp (Variables|Default|GetMeshComp))
  (bind _returnvalue (Transformation|GetSocketLocation _meshcomp _bonename))
  ;[0.15 0.15 0.15 0.5] Check for parry actors
  (Utilities|Array|Clear (Variables|Default|GetParryNotifyActors))
  (bind (_outhits _returnvalue_2) (Collision|MultiSphereTraceForObjects _returnvalue (+ _returnvalue (* (Transformation|GetActorForwardVector (Components|GetOwner)) 5e+01)) 1e+02 (Variables|Default|GetObjectTypes) false (Utilities|Array|MakeArray (Variables|Default|GetOwner)) "None"))
  (if _returnvalue_2
    (for _array_element _outhits
      (if (not (Utilities|Array|ContainsItem (Variables|Default|GetParryNotifyActors) (.HitActor (Collision|BreakHitResult _array_element))))
        (Utilities|Array|AddUnique (Variables|Default|GetParryNotifyActors) (.HitActor (Collision|BreakHitResult _array_element)))))
    (return true)
    (else
      (return false))))

(fn GetParryActors
  (return (Variables|Default|GetParryNotifyActors)))

(fn SetAttackingBoneName
  (params (Bone :type Name :default "None"))
  (Variables|Default|SetBoneName Bone)
  (return true))