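; Player cover component that finds cover in the camera's direction, moves the character to it and handles movement and aiming there.
; Traces measure the surface's height and validate its width, then auto-move runs until arrival or input aborts it.
; A movement plane constraint holds the character to the wall, while traces limit sliding, detect peekable edges and toggle crouch.
; Aiming stands up or sidesteps to peek, and gameplay events signal cover changes.
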(event EventTakeCover
  (bind _returnvalue (Game|GetPlayerCharacter 0))
  (bind _returnvalue_2 (Pawn|GetMovementComponent _returnvalue))
  ;[0.15 0.15 0.15 0.5] Take cover
  (Variables|Default|GetbIsInCover
    (:then)
    (:else
      (bind (_returnvalue_3 _location _normal) (Cover|Trace|CoverTrace))
      (if _returnvalue_3
        (CallFunction|CheckCrouch)
        (Utilities|MovetoCover _location
          (:Completed
            (Class|MovementComponent|SetPlaneConstraintEnabled _returnvalue_2 true)
            (Class|MovementComponent|SetPlaneConstraintNormal _returnvalue_2 _normal)
            (Variables|Default|SetbIsInCover true)
            (Ability|SendGameplayEventtoActor (Components|GetOwner) "(TagName=\"Event.Cover.TakeCover\")")))
        (else
          (Ability|SendGameplayEventtoActor (Components|GetOwner) "(TagName=\"Event.Cover.TakeCover\")"))))))

(event EventExitCover
  ;[0.15 0.15 0.15 0.5] Exit cover
  (Class|MovementComponent|SetPlaneConstraintEnabled (Pawn|GetMovementComponent (Game|GetPlayerCharacter 0)) false)
  (Variables|Default|GetWasCrouching
    (:then
      (if (not (Variables|/Script/Engine.Character|GetbIsCrouched (Game|GetPlayerCharacter 0)))
        (Character|Crouch (Game|GetPlayerCharacter 0))))
    (:else
      (if (Variables|/Script/Engine.Character|GetbIsCrouched (Game|GetPlayerCharacter 0))
        (Character|UnCrouch (Game|GetPlayerCharacter 0)))
      (Variables|Default|SetbIsInCover false)
      (Ability|SendGameplayEventtoActor (Components|GetOwner) "(TagName=\"Event.Cover.ExitCover\")"))))

(event EventBeginPlay
  ;[0.15 0.15 0.15 0.5] Begin play
  (Variables|Default|SetCapsuleCollision (Actor|GetComponentbyClass (Components|GetOwner) "/Script/Engine.CapsuleComponent")))

(fn TraceHeight
  (params (Hit :type Hit%20Result%20Structure%20%28by%20ref%29))
  (bind _absolutevector (Variables|Cover|GetAbsoluteVector))
  (bind (_bblockinghit _binitialoverlap _time _distance _location _impactpoint _normal _impactnormal _physmat _hitactor _hitcomponent) (Collision|BreakHitResult Hit))
  (bind _impactnormal_2 (Collision|BreakHitResult Hit))
  (bind _returnvalue (Math|Vector|CrossProduct _impactnormal_2 _absolutevector))
  (bind _returnvalue_2 (- _impactpoint _impactnormal))
  (bind _returnvalue_3 (Math|Vector|CrossProduct _returnvalue _impactnormal_2))
  (bind _returnvalue_4 (Math|Vector|Normalize _returnvalue_3))
  (bind _returnvalue_5 (* 2e+02 _returnvalue_4))
  (bind _returnvalue_6 (+ _returnvalue_5 _returnvalue_2))
  (bind (_hitlocation _hitnormal _bonename _outhit _returnvalue_7) (Collision|LineTraceComponent _hitcomponent _returnvalue_6 (Math|Vector|Lerp(Vector) _returnvalue_6 _returnvalue_2 1.5) true true true))
  (if _returnvalue_7
    (Variables|Default|SetObjectHeight (Math|Vector|Distance(Vector) (.ImpactPoint (Collision|BreakHitResult Hit)) _hitlocation))
    (return)))

(fn TraceWidth
  (params (Hit :type Hit%20Result%20Structure%20%28by%20ref%29) (AbsoluteVector :type Vector))
  (bind (_bblockinghit _binitialoverlap _time _distance _location _impactpoint _normal _impactnormal _physmat _hitactor _hitcomponent) (Collision|BreakHitResult Hit))
  (bind _returnvalue (/ 7e+01 2.0))
  (bind _returnvalue_2 (* AbsoluteVector _returnvalue))
  (bind _returnvalue_3 (* _impactnormal 37.0))
  (bind _returnvalue_4 (+ _impactpoint _returnvalue_2))
  (bind _returnvalue_5 (Collision|LineTraceComponent _hitcomponent (+ _returnvalue_4 _returnvalue_3) (- _returnvalue_4 _returnvalue_3) false true true))
  (return _returnvalue_5))

(fn CoverTrace
  (bind _returnvalue (Components|GetOwner))
  (bind _returnvalue_2 (Game|GetPlayerCameraManager 0))
  (bind _returnvalue_3 (Camera|GetCameraRotation _returnvalue_2))
  (bind _returnvalue_4 (Transformation|GetActorLocation _returnvalue))
  (bind _returnvalue_5 (Math|Vector|GetForwardVector _returnvalue_3))
  (bind (_outhit _returnvalue_6) (Collision|LineTraceByChannel _returnvalue_4 (+ _returnvalue_4 (* (Math|Vector|MakeVector (.x _returnvalue_5) (.y _returnvalue_5) 0.0) 3e+02)) "TraceTypeQuery1" false 0 "ForDuration"))
  (if _returnvalue_6
    (Variables|Cover|SetAbsoluteVector (* (Math|Vector|GetUpVector (.HitComponent (Collision|BreakHitResult _outhit))) (Math|Float|Sign(Float) (Math|Vector|DotProduct (Math|Vector|GetUpVector (.HitComponent (Collision|BreakHitResult _outhit))) (Transformation|GetActorUpVector (Components|GetOwner))))))
    (Cover|Trace|TraceHeight _outhit)
    (bind _returnvalue_7 (Cover|Trace|TraceWidth _outhit (Math|Vector|CrossProduct (Variables|Cover|GetAbsoluteVector) (.ImpactNormal (Collision|BreakHitResult _outhit)))))
    (if _returnvalue_7
      (bind _returnvalue_8 (Cover|Trace|TraceWidth _outhit (Math|Vector|NegateVector (Math|Vector|CrossProduct (Variables|Cover|GetAbsoluteVector) (.ImpactNormal (Collision|BreakHitResult _outhit))))))
      (if _returnvalue_8
        (return true (.ImpactPoint (Collision|BreakHitResult _outhit)) (.Normal (Collision|BreakHitResult _outhit)))
        (else
          (return false "0, 0, 0" "0, 0, 0")))
      (else
        (return false "0, 0, 0" "0, 0, 0")))
    (else
      (return false "0, 0, 0" "0, 0, 0"))))

(fn CheckCrouch
  (bind _returnvalue (Game|GetPlayerCharacter 0))
  (if (< (Variables|Default|GetObjectHeight) 65.0)
    (bind _output_get (Variables|Default|SetWasCrouching (Variables|/Script/Engine.Character|GetbIsCrouched _returnvalue)))
    (if (not _output_get)
      (Character|Crouch _returnvalue))))

(fn MoveinCover
  (bind _returnvalue (Game|GetPlayerCharacter 0))
  (bind _returnvalue_2 (Components|GetOwner))
  (bind _returnvalue_3 (Components|GetOwner))
  (bind _returnvalue_4 (Game|GetPlayerCharacter 0))
  (bind _returnvalue_5 (Game|GetPlayerCharacter 0))
  (bind _returnvalue_6 (Game|GetPlayerController 0))
  (bind _returnvalue_7 (Game|GetPlayerCharacter 0))
  (bind _returnvalue_8 (Components|GetOwner))
  (bind _returnvalue_9 (Game|GetPlayerCharacter 0))
  (bind _returnvalue_10 (Components|GetOwner))
  (bind _returnvalue_11 (Game|GetPlayerCharacter 0))
  (bind _returnvalue_12 (Pawn|GetMovementComponent _returnvalue_5))
  (bind _returnvalue_13 (Pawn|GetMovementComponent _returnvalue_4))
  (bind _returnvalue_14 (Transformation|GetActorLocation _returnvalue_3))
  (bind _returnvalue_15 (Transformation|GetActorLocation _returnvalue_10))
  (bind _returnvalue_16 (Pawn|GetControlRotation _returnvalue_6 :!class /Script/Engine.Controller))
  (bind _returnvalue_17 (Transformation|GetActorLocation _returnvalue_8))
  (bind _returnvalue_18 (Pawn|GetMovementComponent _returnvalue_9))
  (bind _returnvalue_19 (Transformation|GetActorLocation _returnvalue_2))
  (bind _charactermovement (Variables|/Script/Engine.Character|GetCharacterMovement _returnvalue_11))
  (bind _returnvalue_20 (Class|MovementComponent|GetPlaneConstraintNormal _returnvalue_12))
  (bind _returnvalue_21 (AI|Components|NavMovement|IsCrouching _charactermovement))
  (bind _returnvalue_22 (Class|MovementComponent|GetPlaneConstraintNormal _returnvalue_13))
  (bind _returnvalue_23 (Math|Rotator|MakeRotator 0.0 0.0 (.yaw _returnvalue_16)))
  (bind _returnvalue_24 (Class|MovementComponent|GetPlaneConstraintNormal _returnvalue_18))
  (bind (_x _y _z) (Math|Vector|BreakVector _returnvalue_14))
  (bind _returnvalue_25 (Math|Vector|GetRightVector _returnvalue_23))
  (bind _returnvalue_26 (Math|Rotator|MakeRotfromX _returnvalue_22))
  (bind _returnvalue_27 (* _returnvalue_24 -1.0))
  (bind _returnvalue_28 (* _returnvalue_20 -1.0))
  (bind _returnvalue_29 (Math|Rotator|MakeRotfromX _returnvalue_27))
  (bind _returnvalue_30 (Math|Vector|GetRightVector _returnvalue_26))
  (bind _returnvalue_31 (Math|Vector|GetRightVector _returnvalue_29))
  (bind _returnvalue_32 (* _returnvalue_30 45.0))
  (bind _returnvalue_33 (* _returnvalue_31 45.0))
  (bind _returnvalue_34 (+ _returnvalue_19 _returnvalue_32))
  (bind _returnvalue_35 (+ _returnvalue_17 _returnvalue_33))
  (Utilities|FlowControl|Sequence
    (:then_0
      ;[0.15 0.15 0.15 0.5] Cache move right
      (bind _returnvalue_36 (Class|BPICharacter|GetMoveRight/Left(Message) (Game|GetPlayerCharacter 0)))
      (LocalVariables|SetMoveRight _returnvalue_36))
    (:then_1
      ;[0.15 0.15 0.15 0.5] Perform right trace
      (bind _returnvalue_37 (Collision|LineTraceByChannel _returnvalue_35 (+ _returnvalue_35 (* _returnvalue_27 2e+02)) (Variables|Debug|GetTrace%20Channel) false 0 (Variables|Debug|GetDraw%20Debug%20Type)))
      (bind _output_get (LocalVariables|SetRightHit _returnvalue_37))
      (Variables|Default|SetbCanPeekRight (and (not _output_get) (== (Math|Float|Sign(Float) (LocalVariables|GetMoveRight)) 1.0))))
    (:then_2
      ;[0.15 0.15 0.15 0.5] Perform left trace
      (bind _returnvalue_38 (Collision|LineTraceByChannel _returnvalue_34 (+ _returnvalue_34 (* (* _returnvalue_22 -1.0) 2e+02)) (Variables|Debug|GetTrace%20Channel) false 0 (Variables|Debug|GetDraw%20Debug%20Type)))
      (bind _output_get_2 (LocalVariables|SetLeftHit _returnvalue_38))
      (Variables|Default|SetbCanPeekLeft (and (not _output_get_2) (== (Math|Float|Sign(Float) (LocalVariables|GetMoveRight)) -1.0))))
    (:then_3
      ;[0.15 0.15 0.15 0.5] check if  both right and left trace had a hit and set plane normal to it
      (if (and (LocalVariables|GetRightHit) (LocalVariables|GetLeftHit))
        (bind _returnvalue_39 (Class|BPICharacter|GetMoveRight/Left(Message) (Components|GetOwner)))
        (if (!= _returnvalue_39 0.0)
          (bind (_outhit _returnvalue_40) (Collision|LineTraceByChannel _returnvalue_15 (+ _returnvalue_15 (* (* (Class|MovementComponent|GetPlaneConstraintNormal (Pawn|GetMovementComponent (Game|GetPlayerCharacter 0))) -1.0) 2e+02)) (Variables|Debug|GetTrace%20Channel) false 0 (Variables|Debug|GetDraw%20Debug%20Type)))
          (if _returnvalue_40
            (Class|MovementComponent|SetPlaneConstraintNormal (Pawn|GetMovementComponent (Game|GetPlayerCharacter 0)) (.Normal (Collision|BreakHitResult _outhit)))
            (bind _returnvalue_41 (Class|BPICharacter|GetMoveRight/Left(Message) _returnvalue_7))
            (Pawn|Input|AddMovementInput _returnvalue_7 _returnvalue_25 _returnvalue_41 false)))
        (else
          ;[0.15 0.15 0.15 0.5] allow move if an input is press
          (Pawn|Input|AddMovementInput (Game|GetPlayerCharacter 0) _returnvalue_25 (Math|Float|SelectFloat (LocalVariables|GetMoveRight) 0.0 (and (select (== (Math|Float|Sign(Float) (LocalVariables|GetMoveRight)) 1.0) (LocalVariables|GetRightHit) (LocalVariables|GetLeftHit)) (!= (Math|Float|Sign(Float) (LocalVariables|GetMoveRight)) 0.0))) false))))
    (:then_4
      ;[0.15 0.15 0.15 0.5] Check Height
      (bind _returnvalue_42 (Collision|LineTraceByChannel (+ (Math|Vector|MakeVector _x _y (+ (- _z (.OutHalfHeight (Components|Capsule|GetScaledCapsuleSize (Variables|Default|GetCapsuleCollision)))) 1.7e+02)) (* (Math|Vector|GetRightVector (Math|Rotator|MakeRotfromX (select (== (Math|Float|Sign(Float) (LocalVariables|GetMoveRight)) 1.0) _returnvalue_28 _returnvalue_20))) 2e+01)) (+ (+ (Math|Vector|MakeVector _x _y (+ (- _z (.OutHalfHeight (Components|Capsule|GetScaledCapsuleSize (Variables|Default|GetCapsuleCollision)))) 1.7e+02)) (* (Math|Vector|GetRightVector (Math|Rotator|MakeRotfromX (select (== (Math|Float|Sign(Float) (LocalVariables|GetMoveRight)) 1.0) _returnvalue_28 _returnvalue_20))) 2e+01)) (* _returnvalue_28 2e+02)) (Variables|Debug|GetTrace%20Channel) false 0 (Variables|Debug|GetDraw%20Debug%20Type)))
      (if _returnvalue_42
        (if _returnvalue_21
          (Character|UnCrouch _returnvalue))
        (elif (not _returnvalue_21)
          (Character|Crouch _returnvalue))))))

(fn AiminCover
  (params (IsAiming :type Boolean))
  (Variables|Default|GetbIsInCover
    (:then
      (if IsAiming
        (if (AI|Components|NavMovement|IsCrouching (Variables|/Script/Engine.Character|GetCharacterMovement (Game|GetPlayerCharacter 0)))
          (Character|UnCrouch (Game|GetPlayerCharacter 0))
          (else
            (Variables|Cover|SetLastLocation (Transformation|GetActorLocation (Components|GetOwner)))
            (if (or (Variables|Default|GetbCanPeekRight) (Variables|Default|GetbCanPeekLeft))
              (AI|Navigation|SimpleMovetoLocation (Pawn|GetController (Game|GetPlayerCharacter 0)) (Cover|Aim|GetAimCoverLocation)))))
        (elif (< (Variables|Default|GetObjectHeight) 65.0)
          (Character|Crouch (Game|GetPlayerCharacter 0))
          (else
            (AI|Navigation|SimpleMovetoLocation (Pawn|GetController (Game|GetPlayerCharacter 0)) (Variables|Cover|GetLastLocation))))))
    (:else)))

(fn GetAimCoverLocation
  (bind _returnvalue (Components|GetOwner))
  (bind _returnvalue_2 (Components|GetOwner))
  (bind _returnvalue_3 (Game|GetPlayerCharacter 0))
  (bind _bcanpeekleft (Variables|Default|GetbCanPeekLeft))
  (bind _distance (LocalVariables|GetDIstance))
  (bind _distance_2 (LocalVariables|GetDIstance))
  (bind _returnvalue_4 (Pawn|GetMovementComponent _returnvalue_3))
  (bind _returnvalue_5 (Transformation|GetActorLocation _returnvalue))
  (bind _returnvalue_6 (Transformation|GetActorLocation _returnvalue_2))
  (bind _returnvalue_7 (Class|MovementComponent|GetPlaneConstraintNormal _returnvalue_4))
  (bind _returnvalue_8 (Math|Rotator|MakeRotfromX _returnvalue_7))
  (bind _returnvalue_9 (* _returnvalue_7 -1.0))
  (bind _returnvalue_10 (Math|Vector|GetRightVector _returnvalue_8))
  (bind _returnvalue_11 (Math|Rotator|MakeRotfromX _returnvalue_9))
  (bind _returnvalue_12 (Math|Vector|GetRightVector _returnvalue_11))
  (bind _returnvalue_13 (* _returnvalue_10 _distance))
  (bind _returnvalue_14 (* _returnvalue_12 _distance_2))
  (bind _returnvalue_15 (+ _returnvalue_6 _returnvalue_13))
  (bind _returnvalue_16 (+ _returnvalue_5 _returnvalue_14))
  (bind _returnvalue_17 (select _bcanpeekleft _returnvalue_15 _returnvalue_16))
  (Rendering|Debug|DrawDebugSphere _returnvalue_17 3e+01 12 "(R=1.000000,G=1.000000,B=1.000000,A=1.000000)" 0.0)
  (return _returnvalue_17))