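; Character interaction component that finds an interactable actor through an async targeting preset and acts on its InteractableComponent type.
; Pickups send an equip gameplay event carrying the actor as payload; without a valid target, a generic interact event goes to the owner.
; Mounting sets motion-warp targets from mount sockets, plays montages on character and mount, disables capsule collision, then on a montage notify attaches the character and possesses the mounted pawn.
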(event Custom|Mount
  (bind _returnvalue (Utilities|Name|MakeLiteralName "None"))
  (bind _returnvalue_2 (Utilities|Name|MakeLiteralName "None"))
  ;[0.15 0.15 0.15 0.5] Mount
  (bind _aspawn (Utilities|Casting|CastToPawn (Variables|Default|GetNearstActor)))
  (Variables|Default|SetPawnToMount _aspawn)
  ;;[0.15 0.15 0.15 0.5] Warp to door and seat
  (Variables|Default|SetMountableMesh (Actor|GetComponentbyClass (Variables|Default|GetPawnToMount) "/Script/Engine.SkeletalMeshComponent"))
  (bind _output_get (Variables|Default|SetMotionWarpComp (Actor|GetComponentbyClass (Variables|Default|GetAs%20Character) "/Script/MotionWarping.MotionWarpingComponent")))
  (Class|MotionWarpingComponent|AddorUpdateWarpTargetfromLocationandRotation _output_get "None" (Transformation|GetSocketLocation (Variables|Default|GetMountableMesh) _returnvalue) (Transformation|GetSocketRotation (Variables|Default|GetMountableMesh) _returnvalue))
  (Class|MotionWarpingComponent|AddorUpdateWarpTargetfromLocationandRotation (Variables|Default|GetMotionWarpComp) "None" (Transformation|GetSocketLocation (Variables|Default|GetMountableMesh) _returnvalue_2) (Transformation|GetSocketRotation (Variables|Default|GetMountableMesh) _returnvalue_2))
  ;;[0.15 0.15 0.15 0.5] Play montages and set movement mode
  (Animation|Montage|PlayMontage (Variables|/Script/Engine.Character|GetMesh (Variables|Default|GetAs%20Character)) 0
    (:then
      (bind _notifyname (Animation|Montage|PlayMontage (Variables|Default|GetMountableMesh) 0)
        (:then
          (Collision|SetCollisionEnabled (Variables|/Script/Engine.Character|GetCapsuleComponent (Variables|Default|GetAs%20Character)) "NoCollision")
          (Pawn|Components|CharacterMovement|SetMovementMode (Variables|/Script/Engine.Character|GetCharacterMovement (Variables|Default|GetAs%20Character)) "MOVE_Flying" 0))
        (:OnNotifyBegin
          ;;[0.15 0.15 0.15 0.5] Attach and possess
          (switch name _notifyname
            (:DoorClosed
              (Transformation|AttachActorToActor (Variables|Default|GetAs%20Character) (Variables|Default|GetNearstActor) "None" "KeepWorld" "KeepWorld" "KeepWorld" true)
              (Actor|SetOwner (Variables|Default|GetNearstActor) (Variables|Default|GetAs%20Character))
              (Pawn|Possess (select (Pawn|IsPlayerControlled (Variables|Default|GetPawnToMount)) (Game|GetPlayerController 0) (Pawn|GetController (Variables|Default|GetPawnToMount))) (Variables|Default|GetPawnToMount))
              (Ability|SendGameplayEventtoActor (Variables|Default|GetAs%20Character) "(TagName=\"Event.Interact\")"))))))))

(event EventTryInteract
  ;[0.15 0.15 0.15 0.5] Interact
  (bind _targetinghandle (|PerformTargetingRequest (Components|GetOwner) "/Game/Blueprints/Data/TargetPreset/TP_FindInteractableActors.TP_FindInteractableActors" true)
    (:Targeted
      (Utilities|IsValid (Utilities|Array|Get(acopy) (Class|TargetingSubsystem|GetTargetingResultsActors (GameInstanceSubsystems|GetTargetingSubsystem) _targetinghandle))
        (:Is%20Valid
          (Variables|Default|SetNearstActor (Utilities|Array|Get(acopy) (Class|TargetingSubsystem|GetTargetingResultsActors (GameInstanceSubsystems|GetTargetingSubsystem) _targetinghandle)))
          (Interact|InteractAction))
        (:Is%20Not%20Valid
          (Ability|SendGameplayEventtoActor (Components|GetOwner) "(TagName=\"Event.Interact\")"))))))

(event EventBeginPlay
  ;[0.15 0.15 0.15 0.5] Beginplay
  (bind _ascharacter (Utilities|Casting|CastToCharacter (Components|GetOwner)))
  (Variables|Default|SetAs%20Character _ascharacter))

(fn InteractAction
  (switch Utilities|FlowControl|Switch|SwitchonEInteractableType (Variables|/Script/ProjectGrace.InteractableComponent|GetInteractableType (Actor|GetComponentbyClass (Variables|Default|GetNearstActor) "/Script/ProjectGrace.InteractableComponent"))
    (:Pickup
      (Interact|Type|Pickup))
    (:Mount
      (CallFunction|Mount))))

(fn Pickup
  (bind _returnvalue (Game|ConstructObjectfromClass "/Game/GameplayAbilities/Payloads/OBP_AbilityPayload.OBP_AbilityPayload_C"))
  (Variables|/Game/GameplayAbilities/Payloads/OBP_AbilityPayload.OBP_AbilityPayload_C|SetMessageActor _returnvalue (Variables|Default|GetNearstActor))
  (Ability|SendGameplayEventtoActor (Components|GetOwner) "(TagName=\"Abilities.Item.Equip\")" (Utilities|Struct|MakeGameplayEventData _returnvalue)))