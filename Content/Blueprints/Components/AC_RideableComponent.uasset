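; Actor component that lets its owning Character mount and dismount Rideable items through equip updates.
; Equipping caches the rideable and its movement component, raises the walkable floor angle and disables horizontal ground velocity maintenance, adding a rideable input mapping for players.
; Unequipping clears the ride, restoring input and movement settings only for player-controlled characters.
; Two getters supply foot effector positions from the rideable's mesh sockets, slightly raised.
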(event EventUpdateEquipItem
  (params (IsEquipped :type Boolean) (Item :type Actor%20Object%20Reference))
  (bind _as_character (Variables|Default|GetAs%20Character))
  (bind _as_character_2 (Variables|Default|GetAs%20Character))
  (bind _charactermovement (Variables|/Script/Engine.Character|GetCharacterMovement _as_character))
  (bind _charactermovement_2 (Variables|/Script/Engine.Character|GetCharacterMovement _as_character_2))
  ;[0.15 0.15 0.15 0.5] Mount and umount ride
  (if IsEquipped
    (bind _asrideable (Utilities|Casting|CastToRideable Item))
    (Variables|Default|SetCurrentRideable _asrideable)
    (Variables|Default|SetbHasRide true)
    (Variables|Default|SetRideableMovementComponent (Actor|GetComponentbyClass (Variables|Default|GetCurrentRideable) "/Script/ProjectGrace.RideableMovementComponent"))
    (Pawn|Components|CharacterMovement|SetWalkableFloorAngle _charactermovement_2 8e+01)
    (Variables|/Script/Engine.CharacterMovementComponent|SetbMaintainHorizontalGroundVelocity _charactermovement_2 false)
    (if (Pawn|IsPlayerControlled (Variables|Default|GetAs%20Character))
      (Input|AddMappingContext (PlayerController|LocalPlayerSubsystems|GetEnhancedInputLocalPlayerSubsystem (Game|GetPlayerController 0)) "/Game/Input/IMC_Rideable.IMC_Rideable" 1 "(bIgnoreAllPressedKeysUntilRelease=True,bForceImmediately=False,bNotifyUserSettings=False)"))
    (else
      (Variables|Default|SetbHasRide false)
      (Variables|Default|SetCurrentRideable 0)
      (if (Pawn|IsPlayerControlled (Variables|Default|GetAs%20Character))
        (Input|RemoveMappingContext (PlayerController|LocalPlayerSubsystems|GetEnhancedInputLocalPlayerSubsystem (Game|GetPlayerController 0)) "/Game/Input/IMC_Rideable.IMC_Rideable" "(bIgnoreAllPressedKeysUntilRelease=True,bForceImmediately=False,bNotifyUserSettings=False)")
        (Pawn|Components|CharacterMovement|SetWalkableFloorAngle _charactermovement 45.0)
        (Variables|/Script/Engine.CharacterMovementComponent|SetbMaintainHorizontalGroundVelocity _charactermovement true)))))

(event EventBeginPlay
  ;[0.15 0.15 0.15 0.5] Begin play
  (Variables|Default|SetSkeletalMesh (Actor|GetComponentbyClass (Components|GetOwner) "/Script/Engine.SkeletalMeshComponent"))
  (bind _ascharacter (Utilities|Casting|CastToCharacter (Components|GetOwner)))
  (Variables|Default|SetAs%20Character _ascharacter))

(fn GetLeftFootEffector
  (bind _currentrideable (Variables|Default|GetCurrentRideable)
    (:then
      (return (+ (Transformation|GetSocketLocation (Variables|/Script/ProjectGrace.Rideable|GetMesh _currentrideable) (Variables|/Script/ProjectGrace.Rideable|GetLeftFoot_Marker _currentrideable)) "0.000000,0.000000,10.000000")))
    (:else
      (return "0, 0, 0"))))

(fn GetRightFootEffector
  (bind _currentrideable (Variables|Default|GetCurrentRideable)
    (:then
      (return (+ (Transformation|GetSocketLocation (Variables|/Script/ProjectGrace.Rideable|GetMesh _currentrideable) (Variables|/Script/ProjectGrace.Rideable|GetRightFoot_Marker _currentrideable)) "0.000000,0.000000,10.000000")))
    (:else
      (return "0, 0, 0"))))