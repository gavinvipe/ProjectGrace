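; Actor component that equips, switches and drops a character's items, working with its Inventory component and DT_Items data assets.
; Equipping adds to inventory, async-loads and spawns the item or reuses one from the EquippedItems map, then attaches it and hides the previous one.
; Unequipping removes it from inventory or stack and spawns a pickup ahead of the owner.
; Gameplay events report results; Weapon and Rideable components receive equip updates.
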(event Custom|Attach%20Item%20to%20Socket
  (params (ItemID :type Name) (ShouldSpawn :type Boolean))
  (bind _equippeditems (Variables|Default|GetEquippedItems))
  (bind _owner (Variables|Default|GetOwner))
  (bind (_value _returnvalue) (Utilities|Map|Find _equippeditems ItemID))
  ;[0.15 0.15 0.15 0.5] Attach item
  (Variables|Default|SetIsEquipping true)
  (Equip|HandlePerviousItem)
  (if ShouldSpawn
    ;;[0.15 0.15 0.15 0.5] Spawn, attach and add to equipped items
    (bind _returnvalue_2 (Utilities|GetDataTableRow "/Game/Blueprints/Data/DataTables/DT_Items.DT_Items" ItemID)
      (:then
        (Variables|Default|SetEquippedItemID ItemID)
        (Utilities|AsyncLoadClassAsset (Variables|/Script/ProjectGrace.ItemDataAsset|GetItemClass (Utilities|Struct|BreakInventoryItem _returnvalue_2))
          (:Completed
            (bind _returnvalue_3 (Game|SpawnActorfromClass (Utilities|ResolveSoftReference (Variables|/Script/ProjectGrace.ItemDataAsset|GetItemClass (Utilities|Struct|BreakInventoryItem _returnvalue_2))) (Math|Transform|MakeTransform "0, 0, 0" "0, 0, 0" "1.000000,1.000000,1.000000") "Undefined" "MultiplyWithRoot" (Variables|Default|GetOwner) (Utilities|Struct|BreakInventoryItem _returnvalue_2) 0))
            (Variables|Default|SetCurrentEquippedItem _returnvalue_3)
            (Equip|AttachItem (Utilities|Struct|BreakInventoryItem _returnvalue_2))
            (Utilities|Map|Add (Variables|Default|GetEquippedItems) (Variables|Default|GetEquippedItemID) (Variables|Default|GetCurrentEquippedItem))
            (Ability|SendGameplayEventtoActor _owner "(TagName=\"Event.Item.Equip.Completed\")" :!label _label)
            (Ability|SendGameplayEventtoActor _owner "(TagName=\"Event.Interact\")")
            (Variables|Default|SetIsEquipping false)
            (Equip|UpdateItem true)))))
    (else
      ;;[0.15 0.15 0.15 0.5] find item and attach it
      (if _returnvalue
        (bind _output_get (Variables|Default|SetEquippedItemID ItemID))
        (Variables|Default|SetCurrentEquippedItem _value)
        (bind _returnvalue_4 (Utilities|GetDataTableRow "/Game/Blueprints/Data/DataTables/DT_Items.DT_Items" _output_get)
          (:then
            (Equip|AttachItem (Utilities|Struct|BreakInventoryItem _returnvalue_4))
            (Rendering|SetActorHiddenInGame (Variables|Default|GetCurrentEquippedItem) false)
            (goto _label)))))))

(event Custom|Spawn%20Pickup
  (params (ItemID :type Name) (ShouldDestroyItem :type Boolean))
  (bind _owner (Variables|Default|GetOwner))
  (bind _equippeditems (Variables|Default|GetEquippedItems))
  (bind (_value _returnvalue) (Utilities|Map|Find _equippeditems ItemID))
  ;[0.15 0.15 0.15 0.5] Spawn Pickup
  (Variables|Default|SetIsUnEquipping true)
  (bind _returnvalue_2 (Utilities|GetDataTableRow "/Game/Blueprints/Data/DataTables/DT_Items.DT_Items" ItemID)
    (:then
      (Utilities|AsyncLoadAsset (Variables|/Script/ProjectGrace.ItemDataAsset|GetPickupMesh (Utilities|Struct|BreakInventoryItem _returnvalue_2))
        (:Completed
          (bind _returnvalue_3 (Game|SpawnActorfromClass "/Script/ProjectGrace.Pickup" (Math|Transform|MakeTransform (+ (Transformation|GetActorLocation _owner) (* (Transformation|GetActorForwardVector _owner) (Variables|Default|GetUnequipSpawnDistance))) "0, 0, 0" "1.000000,1.000000,1.000000") "Undefined" "MultiplyWithRoot" 0 0))
          (Variables|/Script/ProjectGrace.InteractableComponent|SetItemID (Variables|/Script/ProjectGrace.Pickup|GetInteractableComponent _returnvalue_3) (Utilities|Struct|MakeDataTableRowHandle "/Game/Blueprints/Data/DataTables/DT_Items.DT_Items" ItemID))
          (Components|StaticMesh|SetStaticMesh (Variables|/Script/ProjectGrace.Pickup|GetPickupMesh _returnvalue_3) (Utilities|ResolveSoftReference (Variables|/Script/ProjectGrace.ItemDataAsset|GetPickupMesh (Utilities|Struct|BreakInventoryItem _returnvalue_2))))
          ;;[0.15 0.15 0.15 0.5] Destroys and remove current item
          (if ShouldDestroyItem
            (if _returnvalue
              (Actor|DestroyActor _value))
            (Utilities|Map|Remove (Variables|Default|GetEquippedItems) ItemID)
            (Ability|SendGameplayEventtoActor (Variables|Default|GetOwner) "(TagName=\"Event.Item.Unequip.Completed\")")
            (Variables|Default|SetIsUnEquipping false)
            (Equip|UpdateItem false)
            (else
              (Ability|SendGameplayEventtoActor (Variables|Default|GetOwner) "(TagName=\"Event.Item.Unequip.Completed\")"))))))))

(event EventBeginPlay
  ;[0.15 0.15 0.15 0.5] Begin play
  (bind _output_get (Variables|Default|SetOwner (Components|GetOwner)))
  (Variables|Default|SetInventoryComp (Actor|GetComponentbyClass _output_get "/Script/ProjectGrace.InventoryComponent"))
  (Variables|Default|SetMesh (Actor|GetComponentbyClass (Variables|Default|GetOwner) "/Script/Engine.SkeletalMeshComponent"))
  (Variables|Default|SetWeaponComp (Actor|GetComponentbyClass (Variables|Default|GetOwner) "/Script/ProjectGrace.WeaponComponent"))
  (Variables|Default|SetRideableComp (Actor|GetComponentbyClass (Variables|Default|GetOwner) "/Script/ProjectGrace.RideableComponent")))

(event EventUseStackItem
  ;[0.15 0.15 0.15 0.5] Remove from stack
  (Class|EquipComponent|UnequipItem (Variables|Default|GetEquippedItemID)))

(event EventSwitchItem
  (params (ItemID :type Name :default "None"))
  ;[0.15 0.15 0.15 0.5] Switch Item
  (if (.ReturnValue (Utilities|Map|Find (Variables|Default|GetEquippedItems) ItemID))
    (CallFunction|AttachItemtoSocket ItemID false)
    (else
      (Equip|HandlePerviousItem)
      (Equip|UpdateItem false))))

(event EventEquipItem
  (params (ItemID :type Name :default "None") (ItemPickup :type Actor%20Object%20Reference))
  ;[0.15 0.15 0.15 0.5] Equip Item
  (Utilities|IsValid ItemPickup
    (:Is%20Valid
      (bind _returnvalue (Class|InteractInterface|GetInteractableItemID(Message) ItemPickup))
      (Equip|AddItem _returnvalue ItemPickup))
    (:Is%20Not%20Valid
      (Equip|AddItem ItemID))))

(event EventUnequipItem
  (params (ItemID :type Name :default "None"))
  (bind _equippeditemid (Variables|Default|GetEquippedItemID))
  ;[0.15 0.15 0.15 0.5] Unequip
  (if (== ItemID "")
    (Variables|Default|GetCurrentEquippedItem
      (:then
        (bind _returnvalue (Equip|RemoveItem (Variables|Default|GetEquippedItemID)))
        (switch Utilities|FlowControl|Switch|SwitchonEInventoryRemMsg _returnvalue
          (:Inventory
            (CallFunction|SpawnPickup _equippeditemid true))
          (:Stack
            (CallFunction|SpawnPickup _equippeditemid false))))
      (:else
        (Ability|SendGameplayEventtoActor (Variables|Default|GetOwner) "(TagName=\"Event.Item.Unequip.Completed\")")))
    (else
      (bind _returnvalue_2 (Equip|RemoveItem ItemID))
      (switch Utilities|FlowControl|Switch|SwitchonEInventoryRemMsg _returnvalue_2
        (:Inventory
          (CallFunction|SpawnPickup ItemID true))
        (:Stack
          (CallFunction|SpawnPickup ItemID false))))))

(fn AddItem
  (params (ItemID :type Name) (Pickup :type Actor%20Object%20Reference))
  (bind _returnvalue (Class|InventoryComponent|AddtoInventory (Variables|Default|GetInventoryComp) ItemID))
  (switch Utilities|FlowControl|Switch|SwitchonEInventoryAddMsg _returnvalue
    (:Inventory
      (CallFunction|AttachItemtoSocket ItemID true)
      (bind _pickup (LocalVariables|GetPickup :!label _label)
        (:then
          (Actor|DestroyActor _pickup))
        (:else)))
    (:Stack
      (CallFunction|AttachItemtoSocket ItemID false)
      (goto _label))
    (:Full
      (Ability|SendGameplayEventtoActor (Components|GetOwner) "(TagName=\"Event.Interact\")"))))

(fn RemoveItem
  (params (ItemID :type Name))
  (bind _returnvalue (Class|InventoryComponent|RemovefromInventory (Variables|Default|GetInventoryComp) ItemID))
  (return _returnvalue))

(fn HandlePerviousItem
  (bind _currentequippeditem (Variables|Default|GetCurrentEquippedItem)
    (:then
      (Rendering|SetActorHiddenInGame _currentequippeditem true)
      (Transformation|AttachComponentToComponent _currentequippeditem (Variables|Default|GetMesh) (Variables|Default|GetPreviousItemSocket) "SnapToTarget" "SnapToTarget" "SnapToTarget" true)
      (Variables|Default|SetCurrentEquippedItem 0))
    (:else)))

(fn GetEquipedItemId
  (params (Item :type Actor%20Object%20Reference))
  (bind (_keypin _valuepin) (Utilities|Map|ForEachLoop(Map) (Variables|Default|GetEquippedItems) :!label _label)
    (:then
      (if (== _valuepin Item)
        (LocalVariables|SetKey _keypin)
        (goto _label BreakPin)))
    (:CompletedPin
      (return (LocalVariables|GetKey)))))

(fn AttachItem
  (params (DataAsset :type Item%20Data%20Asset%20Object%20Reference))
  (Transformation|AttachComponentToComponent (Variables|Default|GetCurrentEquippedItem) (select (Variables|/Script/ProjectGrace.ItemDataAsset|GetbShouldAttachToMesh DataAsset) (Variables|Default|GetMesh) (Class|Actor|FindComponentbyTag (Components|GetOwner) "/Script/Engine.SceneComponent" (Variables|/Script/ProjectGrace.ItemDataAsset|GetComponentTag DataAsset))) (Variables|/Script/ProjectGrace.ItemDataAsset|GetSocketToAttach DataAsset) "SnapToTarget" "SnapToTarget" "SnapToTarget" true))

(fn UpdateItem
  (params (IsEquipped :type Boolean))
  (bind _currentequippeditem (Variables|Default|GetCurrentEquippedItem))
  (if IsEquipped
    (Class|BPIEquip|UpdateEquipItem(Message) (Variables|Default|GetWeaponComp) true _currentequippeditem)
    (Class|BPIEquip|UpdateEquipItem(Message) (Variables|Default|GetRideableComp) true _currentequippeditem)
    (else
      (Class|BPIEquip|UpdateEquipItem(Message) (Variables|Default|GetWeaponComp) false)
      (Class|BPIEquip|UpdateEquipItem(Message) (Variables|Default|GetRideableComp) false))))