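; Melee weapon actor that plays an attack montage and applies damage and hit reactions to struck actors.
; Loads its mesh from an item data asset; Fire async-plays MeleeAnim and sends a fire event when it ends.
; ApplyEffect hits each GAS actor once, sending a random Chooser-picked reaction, fixed SetByCaller damage and a GameplayCue.
; Motion warping is stubbed: the "Melee" target is zeroed and the computed warp location is unused.
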(event EventApplyEffect
  ;[0.15 0.15 0.15 0.5] Apply Gameplay Effects
  (for _array_element (Variables|Default|GetHitResults)
    (Utilities|IsValid (Ability|GetAbilitySystemComponent (.HitActor (Collision|BreakHitResult _array_element)))
      (:Is%20Valid
        (if (not (Utilities|Array|ContainsItem (Variables|Default|GetHitActors) (.HitActor (Collision|BreakHitResult _array_element))))
          (Utilities|Array|AddUnique (Variables|Default|GetHitActors) (.HitActor (Collision|BreakHitResult _array_element)))
          (bind _anim (Utilities|GetHitReactionAnim)
            (:Completed
              (Melee|ActivateHitReaction _array_element _anim)
              (bind _returnvalue (Ability|GameplayEffect|AssignTagSetbyCallerMagnitude (GameplayEffects|MakeOutgoingSpec :self (Ability|GetAbilitySystemComponent (.HitActor (Collision|BreakHitResult _array_element))) :GameplayEffectClass "/Game/GameplayAbilities/Effects/GE_InstantDamage.GE_InstantDamage_C") "(TagName=\"Data.Damage.Instant\")" -15.0))
              (GameplayEffects|ApplyGameplayEffectSpecToSelf (Ability|GetAbilitySystemComponent (.HitActor (Collision|BreakHitResult _array_element))) _returnvalue)
              (GameplayCue|ExecuteGameplayCueOnActor(Burst) (.HitActor (Collision|BreakHitResult _array_element)) (Variables|/Script/ProjectGrace.WeaponDataAsset|GetGameplayCueTag (Variables|Default|GetDataAsset)) (GameplayCue|MakeGameplayCueParametersfromHitResult _array_element))
              (CallFunction|AddGameplayTag (Components|GetOwner) "(TagName=\"Status.Attack.IsUnderAttack.Melee\")"))))))))

(event EventFire
  (bind _meleeanim (Variables|Default|GetMeleeAnim))
  ;[0.15 0.15 0.15 0.5] Fire
  (Class|MotionWarpingComponent|AddorUpdateWarpTargetfromLocationandRotation (Variables|Default|GetMotionWarp) "Melee" "0, 0, 0" "0, 0, 0")
  (Utilities|AsyncLoadAsset _meleeanim
    (:Completed
      (Animation|Montage|PlayMontage (Variables|Default|GetMesh) (Utilities|ResolveSoftReference _meleeanim)
        (:OnCompleted
          _)
        (:OnInterrupted
          _))
      (Ability|SendGameplayEventtoActor (Components|GetOwner) "(TagName=\"Event.Combat.Weapon.Fire\")"))))

(event EventBeginPlay
  ;[0.15 0.15 0.15 0.5] Begin play
  (bind _itemdataasset (Variables|Default|GetItemDataAsset)
    (:then
      (bind _itemstaticmesh (Variables|/Script/ProjectGrace.ItemDataAsset|GetItemStaticMesh _itemdataasset)
        (:then
          (Utilities|AsyncLoadAsset _itemstaticmesh
            (:Completed
              (Components|StaticMesh|SetStaticMesh (Variables|Default|GetStaticMeshComponent) (Utilities|ResolveSoftReference _itemstaticmesh))
              (Variables|Default|SetMesh (Actor|GetComponentbyClass (Components|GetOwner) "/Script/Engine.SkeletalMeshComponent"))
              (Variables|Default|SetMotionWarp (Actor|GetComponentbyClass (Components|GetOwner) "/Script/MotionWarping.MotionWarpingComponent")))))
        (:else)))
    (:else)))

(fn ConstructionScript)

(fn ActivateHitReaction
  (params (HitResult :type Hit%20Result%20Structure%20%28by%20ref%29) (Montage :type Anim%20Montage%20Object%20Reference))
  (bind (_bblockinghit _binitialoverlap _time _distance _location _impactpoint _normal _impactnormal _physmat _hitactor _hitcomponent _hitbonename) (Collision|BreakHitResult HitResult))
  (bind _returnvalue (Game|ConstructObjectfromClass "/Game/GameplayAbilities/Payloads/OBP_AbilityPayload.OBP_AbilityPayload_C"))
  (bind _output_get (LocalVariables|SetAbilityPayload _returnvalue))
  (Variables|/Game/GameplayAbilities/Payloads/OBP_AbilityPayload.OBP_AbilityPayload_C|SetMessageVector _output_get (* (Math|Vector|GetUnitDirection(Vector) (Transformation|GetActorLocation (Components|GetOwner)) _impactpoint) 2e+03))
  (Variables|/Game/GameplayAbilities/Payloads/OBP_AbilityPayload.OBP_AbilityPayload_C|SetMessageName (LocalVariables|GetAbilityPayload) _hitbonename)
  (Ability|SendGameplayEventtoActor _hitactor "(TagName=\"Event.HitReaction\")" (Utilities|Struct|MakeGameplayEventData "(TagName=\"\")" 0 0 (LocalVariables|GetAbilityPayload))))

(fn GetWarpLocationandRotation
  (params (Target :type Actor%20Object%20Reference))
  (return (+ (* (Math|Vector|Normalize (- (Transformation|GetActorLocation (Components|GetOwner)) (Transformation|GetActorLocation Target))) 5e+01) (Transformation|GetActorLocation Target)) (Math|Rotator|FindLookatRotation (Transformation|GetActorLocation (Components|GetOwner)) (Transformation|GetActorLocation Target))))

(fn GetProjectileClass
  (return 0))

(fn GetProjectileMesh
  (return 0))

(fn MeleeTrace
  (Class|Weapon|WeaponTrace)
  (return true))