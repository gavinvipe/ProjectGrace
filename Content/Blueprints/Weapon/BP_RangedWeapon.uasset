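; Ranged weapon Blueprint that loads its skeletal mesh asynchronously and fires as hitscan or projectile.
; Fire checks ammo, plays a montage and traces; the projectile branch async-loads class and mesh, then spawns with trace-aimed, randomly offset velocity.
; Both branches apply GAS SetByCaller damage to the traced actor immediately, even for projectiles, plus a hit cue, owner fire event and tag.
; Failed ammo checks tag the owner LowAmmo.
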(event Custom|ApplyEffects
  (bind _hitresult (Variables|Default|GetHitResult))
  (bind _hitactor (Collision|BreakHitResult _hitresult))
  (bind _returnvalue (Ability|GetAbilitySystemComponent _hitactor))
  ;[0.15 0.15 0.15 0.5] Apply Gameplay Effects
  (Utilities|IsValid _returnvalue
    (:Is%20Valid
      (bind _returnvalue_2 (Ability|GameplayEffect|AssignTagSetbyCallerMagnitude (GameplayEffects|MakeOutgoingSpec :self _returnvalue :GameplayEffectClass "/Game/GameplayAbilities/Effects/GE_InstantDamage.GE_InstantDamage_C") "(TagName=\"Data.Damage.Instant\")" (Variables|Default|GetWeaponDamage)))
      (GameplayEffects|ApplyGameplayEffectSpecToSelf _returnvalue _returnvalue_2))
    (:Is%20Not%20Valid
      _))
  (GameplayCue|ExecuteGameplayCueOnActor(Burst) _hitactor "(TagName=\"GameplayCue.Hit.Shoot\")" (GameplayCue|MakeGameplayCueParametersfromHitResult (Variables|Default|GetHitResult)))
  (Ability|SendGameplayEventtoActor (Components|GetOwner) "(TagName=\"Event.Combat.Weapon.Fire\")")
  (CallFunction|AddGameplayTag (Components|GetOwner) "(TagName=\"Status.Attack.IsUnderAttack.Fire\")"))

(event EventBeginPlay
  ;[0.15 0.15 0.15 0.5] Begin play
  (bind _itemdataasset (Variables|Default|GetItemDataAsset)
    (:then
      (bind _itemskeletalmesh (Variables|/Script/ProjectGrace.ItemDataAsset|GetItemSkeletalMesh _itemdataasset)
        (:then
          (Utilities|AsyncLoadAsset _itemskeletalmesh
            (:Completed
              (Components|SkeletalMesh|SetSkeletalMeshAsset (Variables|Default|GetSkeletalMeshComponent) (Utilities|ResolveSoftReference _itemskeletalmesh))
              (Variables|Default|SetMesh (Actor|GetComponentbyClass (Components|GetOwner) "/Script/Engine.SkeletalMeshComponent")))))
        (:else)))
    (:else)))

(event EventFire
  ;[0.15 0.15 0.15 0.5] Fire
  (if (Class|RangedWeapon|CheckAmmo)
    (Animation|Montage|PlayMontage (Variables|Default|GetMesh) (Variables|Default|GetMontage%20to%20Play)
      (:then
        (Class|RangedWeapon|ConsumeAmmo)
        (Variables|Default|GetbIsHitscan
          (:then
            (Class|Weapon|WeaponTrace)
            (CallFunction|ApplyEffects))
          (:else
            ;;[0.15 0.15 0.15 0.5] Projectile
            (Class|Weapon|WeaponTrace)
            (Collision|LineTraceByChannel (Transformation|GetSocketLocation (Variables|Default|GetWeaponMesh) (Variables|Default|GetTracePoint)) (CallFunction|GetVelocity) "TraceTypeQuery1" false (Utilities|Array|MakeArray (Components|GetOwner)) "ForDuration" true "(R=0.453164,G=0.920433,B=1.000000,A=1.000000)" "(R=0.035079,G=0.200597,B=1.000000,A=1.000000)")
            (bind _projectileclass (Variables|Default|GetProjectileClass)
              (:then
                (Utilities|AsyncLoadClassAsset _projectileclass
                  (:Completed
                    (bind _projectilemesh (Variables|/Script/ProjectGrace.RangedDataAsset|GetProjectileMesh (Variables|Default|GetDataAsset))
                      (:then
                        (Utilities|AsyncLoadAsset _projectilemesh
                          (:Completed
                            (Game|SpawnActorfromClass (Utilities|ResolveSoftReference _projectileclass) (Math|Transform|MakeTransform (Transformation|GetSocketLocation (Variables|Default|GetWeaponMesh) (Variables|Default|GetTracePoint)) "0, 0, 0" "1.000000,1.000000,1.000000") "Undefined" "MultiplyWithRoot" (Components|GetOwner) (Utilities|ResolveSoftReference _projectilemesh) (CallFunction|GetVelocity) 0)
                            (CallFunction|ApplyEffects))))
                      (:else
                        (Class|DebugFunctionLibrary|DebugPrint "Weapon" "ProjectileMesh is not valid" "Warning" true true 5.0 false "None"))))))
              (:else
                (Class|DebugFunctionLibrary|DebugPrint "Weapon" "ProjectileClass is not valid" "Warning" true true 5.0 false "None")))))))
    (else
      (CallFunction|AddGameplayTag (Components|GetOwner) "(TagName=\"Status.Weapon.LowAmmo\")")
      (Class|DebugFunctionLibrary|DebugPrint "Weapon" "Low Ammo!" "Warning" (CallFunction|GetEnablePrintscreen) (CallFunction|GetEnableLog) 5.0 true "None"))))

(fn ConstructionScript)

(fn GetVelocity
  (bind _returnvalue (Math|Random|RandomFloatinRange 2e+02 2.5e+02))
  (bind _tracepoint (Variables|Default|GetTracePoint))
  (bind _hitresult (Variables|Default|GetHitResult))
  (bind _weaponmesh (Variables|Default|GetWeaponMesh))
  (bind _returnvalue_2 (Transformation|GetSocketLocation _weaponmesh _tracepoint))
  (return (+ _returnvalue_2 (* (Math|Vector|Normalize (- (Math|Vector|SelectVector (.impactpoint _hitresult) (.traceend _hitresult) (.bblockinghit _hitresult)) _returnvalue_2)) (Variables|Default|GetProjectileSpeed)) (Math|Vector|MakeVector _returnvalue _returnvalue _returnvalue))))