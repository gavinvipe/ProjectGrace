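; BP_WeaponProjectile is a weapon projectile actor that triggers a gameplay cue after hitting something.
; On BeginPlay it applies its Velocity variable to ProjectileMovement and activates that component.
; A collision hit starts a FuseTime delay, then executes the configured GameplayCueTag on the owning actor with parameters built from the hit result, prints Weapon debug output and destroys the projectile.
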(event OnComponentHit(ProjectileCollision)
  (params (HitComponent :type Primitive%20Component%20Object%20Reference) (OtherActor :type Actor%20Object%20Reference) (OtherComp :type Primitive%20Component%20Object%20Reference) (NormalImpulse :type Vector :default "0, 0, 0") (Hit :type Hit%20Result%20Structure%20%28by%20ref%29))
  (Utilities|FlowControl|Delay (Variables|Default|GetFuseTime))
  (GameplayCue|ExecuteGameplayCueOnActor(Burst) (Components|GetOwner) (Variables|Weapon|Explosive|GetGameplay%20Cue%20Tag) (GameplayCue|MakeGameplayCueParametersfromHitResult Hit))
  (Class|DebugFunctionLibrary|DebugPrint "Weapon" "Projectile Hit!" "Info" (CallFunction|GetEnablePrintscreen) (CallFunction|GetEnableLog) 3.0 true "None")
  (Actor|DestroyActor))

(event EventBeginPlay
  ;[0.15 0.15 0.15 0.5] Begin play
  (Variables|/Script/Engine.MovementComponent|SetVelocity (Variables|Default|GetProjectileMovement) (Variables|Default|GetVelocity))
  (Components|Activation|Activate (Variables|Default|GetProjectileMovement) false))

(fn ConstructionScript)