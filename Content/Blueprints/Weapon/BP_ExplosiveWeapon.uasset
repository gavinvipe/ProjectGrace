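; Explosive weapon Blueprint for thrown weapons, supplying a projectile class and a projectile mesh from its data asset.
; On BeginPlay it async-loads and applies the item's static mesh, then caches the owner's skeletal mesh.
; Fire async-loads and plays the throw montage on that mesh, sending the Event.Combat.Weapon.Fire gameplay event to the owner when the montage completes or is interrupted.
; Melee tracing always returns false.
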(event EventBeginPlay
  ;[0.15 0.15 0.15 0.5] Beginplay
  (bind _itemdataasset (Variables|Default|GetItemDataAsset)
    (:then
      (bind _itemstaticmesh (Variables|/Script/ProjectGrace.ItemDataAsset|GetItemStaticMesh _itemdataasset)
        (:then
          (Utilities|AsyncLoadAsset _itemstaticmesh
            (:Completed
              (Components|StaticMesh|SetStaticMesh (Variables|Default|GetStaticMeshComponent) (Utilities|ResolveSoftReference _itemstaticmesh))
              (Variables|Default|SetMeshComp (Actor|GetComponentbyClass (Components|GetOwner) "/Script/Engine.SkeletalMeshComponent")))))
        (:else)))
    (:else)))

(event EventFire
  (bind _throwanim (Variables|Default|GetThrowAnim))
  ;[0.15 0.15 0.15 0.5] Fire
  (Utilities|AsyncLoadAsset _throwanim
    (:Completed
      (Animation|Montage|PlayMontage (Variables|Default|GetMeshComp) (Utilities|ResolveSoftReference _throwanim)
        (:OnCompleted
          _)
        (:OnInterrupted
          _))
      (Ability|SendGameplayEventtoActor (Components|GetOwner) "(TagName=\"Event.Combat.Weapon.Fire\")"))))

(fn ConstructionScript)

(fn GetProjectileClass
  (return (Variables|Default|GetProjectileClass)))

(fn GetProjectileMesh
  (return (Variables|/Script/ProjectGrace.ExplosiveDataAsset|GetProjectileMesh (Variables|Default|GetDataAsset))))

(fn MeleeTrace
  (return false))