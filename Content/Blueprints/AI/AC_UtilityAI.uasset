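; Utility AI component that reacts to damage and sight perception by choosing and running the owner's highest-scoring task.
; The perception handler passes each stimulus to both sense functions, which filter by sense class, execute the selected task and debug-print its name and score.
; Damage requires a successful stimulus, while sight reacts to gain and loss alike.
; BeginPlay is empty; the code that caches the AIController and binds perception is disconnected.
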(event Custom|TargetPerceptionUpdated
  (params (Actor :type Actor%20Object%20Reference) (Stimulus :type AI%20Stimulus%20Structure))
  (Utilities|FlowControl|Sequence
    (:then_0
      (Sense|SenseDamage Actor Stimulus))
    (:then_1
      (Sense|SenseSight Actor Stimulus))))

(event EventBeginPlay
  ;[0.15 0.15 0.15 0.5] Begin play
)

(fn SenseDamage
  (params (SensedActor :type Actor%20Object%20Reference) (Stimulus :type AI%20Stimulus%20Structure))
  (bind _returnvalue (Class|AIPerceptionSystem|GetSenseClassforStimulus Stimulus))
  (if (== _returnvalue "/Script/AIModule.AISense_Damage")
    (if (.bsuccessfullysensed Stimulus)
      (bind (_selectedtask _score) (Class|UtilityAIComponent|FindHighestScoreTask (Utilities|Struct|MakeUtilityContext (Variables|Default|GetAIController) (Components|GetOwner) 0)))
      (Utilities|IsValid _selectedtask
        (:Is%20Valid
          (Class|UtilityTask|ExecuteTask _selectedtask)
          (Class|DebugFunctionLibrary|DebugPrint "Utility AI" (Utilities|String|ToString(Text) (Utilities|Text|FormatText " 
Current Task: {Task} 
Name: {Name} 
Score: {Score}" (Utilities|GetDisplayName _selectedtask) (GameplayTags|GetTagName (Variables|/Script/ProjectGrace.UtilityTask|GetTag _selectedtask)) _score)) "Success" true false 5.0 true "None"))))))

(fn SenseSight
  (params (SensedActor :type Actor%20Object%20Reference) (Stimulus :type AI%20Stimulus%20Structure))
  (bind _returnvalue (Class|AIPerceptionSystem|GetSenseClassforStimulus Stimulus))
  (if (== _returnvalue "/Script/AIModule.AISense_Sight")
    (bind (_selectedtask _score) (Class|UtilityAIComponent|FindHighestScoreTask (Utilities|Struct|MakeUtilityContext (Variables|Default|GetAIController) (Components|GetOwner) 0)))
    (Utilities|IsValid _selectedtask
      (:Is%20Valid
        (Class|UtilityTask|ExecuteTask _selectedtask)
        (Class|DebugFunctionLibrary|DebugPrint "Utility AI" (Utilities|String|ToString(Text) (Utilities|Text|FormatText " 
Current Task: {Task} 
Name: {Name} 
Score: {Score}" (Utilities|GetDisplayName _selectedtask) (GameplayTags|GetTagName (Variables|/Script/ProjectGrace.UtilityTask|GetTag _selectedtask)) _score)) "Success" true false 5.0 true "None")))))