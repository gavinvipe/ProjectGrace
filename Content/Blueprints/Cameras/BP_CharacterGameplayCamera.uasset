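; Gameplay camera for a character that tracks the current camera mode, style and shoulder side, starting from configurable defaults.
; View changes cycle third-person Close, Balanced and Far, then first person, then back to Close.
; Aiming switches between third-person and aim modes unless in first person, and mode changes fire a settings-changed call.
; Each tick writes the owner's forward vector into a Gameplay Cameras variable.
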(event EventBeginPlay
  (Camera|ChangeCameraMode (Variables|Camera|GetDefaultCameraMode))
  (Camera|ChangeCameraSide (Variables|Camera|GetDefaultCameraSide))
  (Camera|ChangeCameraStyle (Variables|Camera|GetDefaultCameraStyle)))

(event EventTick
  (params (DeltaSeconds :type Float%20%28single-precision%29))
  (Class|BlueprintCameraVariableTableFunctionLibrary|SetVector3CameraVariable (Class|GameplayCameraComponentBase|GetInitialResult) "/Game/Blueprints/Cameras/Data/CV_CameraVar.CV_CameraVar.Vector3dCameraVariable_0" (Transformation|GetActorForwardVector (Components|GetOwner))))

(fn ChangeCameraMode
  (params (CurrentCameraMode :type E_CameraMode%20Enum :default "NewEnumerator0"))
  (Variables|Camera|SetCurrentCameraMode CurrentCameraMode)
  (Default|CallCameraSettingsChanged))

(fn ChangeCameraStyle
  (params (CameraStyle :type E_CameraStyle%20Enum :default "NewEnumerator0"))
  (Variables|Camera|SetCurrentCameraStyle CameraStyle))

(fn ChangeCameraSide
  (params (CameraSide :type E_CameraSide%20Enum :default "NewEnumerator0"))
  (Variables|Camera|SetCurrentCameraSide CameraSide))

(fn ChangeCameraView
  (if (Utilities|Enum|Equal(Enum) (Variables|Camera|GetCurrentCameraMode) "NewEnumerator1")
    (if (Utilities|Enum|Equal(Enum) (Variables|Camera|GetCurrentCameraStyle) "NewEnumerator0")
      (Camera|ChangeCameraMode (select (Camera|IsFirstPerson) "NewEnumerator1" "NewEnumerator0"))
      (else
        (Camera|ChangeCameraStyle (Utilities|Select :Index (Variables|Camera|GetCurrentCameraStyle) :NewEnumerator0 "NewEnumerator0" :NewEnumerator1 "NewEnumerator0" :NewEnumerator2 "NewEnumerator1"))
        (Default|CallCameraSettingsChanged)))
    (Debug|Debug)
    (else
      (Camera|ChangeCameraStyle "NewEnumerator2")
      (Camera|ChangeCameraMode "NewEnumerator1")
      (Debug|Debug))))

(fn IsFirstPerson
  (return (Utilities|Enum|Equal(Enum) (Variables|Camera|GetCurrentCameraMode) "NewEnumerator0")))

(fn Debug
  (bind _currentcameramode (Variables|Camera|GetCurrentCameraMode))
  (Class|DebugFunctionLibrary|DebugPrint "Camera" (Utilities|String|ToString(Text) (Utilities|Text|FormatText " 
Camera Mode: {Mode} 
Camera Style: {Style} 
Camera Side: {Side}" (Utilities|String|EnumtoString _currentcameramode) (Utilities|String|SelectString (Utilities|String|EnumtoString (Variables|Camera|GetCurrentCameraStyle)) "None" (Utilities|Enum|Equal(Enum) _currentcameramode "NewEnumerator1")) (Utilities|String|SelectString (Utilities|String|EnumtoString (Variables|Camera|GetCurrentCameraSide)) "None" (Utilities|Enum|Equal(Enum) (Variables|Camera|GetCurrentCameraMode) "NewEnumerator2")))) "Info" true true 5.0 true "None"))

(fn ChangeCameratoAim
  (params (IsAiming :type Boolean))
  (bind _output_get (Variables|Camera|SetWantsToAim IsAiming))
  (if _output_get
    (if (Camera|IsFirstPerson)
      _
      (else
        (Camera|ChangeCameraMode "NewEnumerator2")))
    (Default|CallCameraSettingsChanged)
    (else
      (if (Camera|IsFirstPerson)
        _
        (else
          (Camera|ChangeCameraMode "NewEnumerator1")))
      (Default|CallCameraSettingsChanged))))